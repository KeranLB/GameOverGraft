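; BP_StateButton is a tactical map button Blueprint that sets the visual state of a referenced Camp to safe, attack or destroy.
; Its Interact function stores the given button name and, if Camp is valid, switches on it to apply the matching material to Camp's first slot.
; Each state change also prints a debug string, and the event graph holds no logic.
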(event EventBeginPlay)

(event Collision|EventActorBeginOverlap
  (params (OtherActor :type Actor%20Object%20Reference)))

(event EventTick
  (params (DeltaSeconds :type Float%20%28single-precision%29)))

(fn ConstructionScript)

(fn Interact
  (params (ButtonName :type String))
  (LocalVariables|SetName ButtonName)
  (bind _camp (Variables|Default|GetCamp)
    (:then
      (switch string (LocalVariables|GetName)
        (:SM_SafeButton
          (Rendering|Material|SetMaterial _camp 0 (Variables|Default|GetM_Safe))
          (Development|PrintString "Button Safe"))
        (:SM_AtkButton
          (Rendering|Material|SetMaterial _camp 0 (Variables|Default|GetM_ATK))
          (Development|PrintString "Button ATK"))
        (:SM_DestroyButton
          (Rendering|Material|SetMaterial _camp 0 (Variables|Default|GetM_Destroy))
          (Development|PrintString "Button Destroy"))))
    (:else)))