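; BP_MapTactic is a tactical map actor that feeds data to a StateButtons object.
; On BeginPlay it copies the world locations of its start and end raycast markers into StateButtons.
; A capsule overlap stores the overlapping static mesh component as StateButtons.Camp and clears it when a static mesh leaves.
; Debug prints report each step.
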(event OnComponentBeginOverlap(Capsule)
  (params (OverlappedComponent :type Primitive%20Component%20Object%20Reference) (OtherActor :type Actor%20Object%20Reference) (OtherComp :type Primitive%20Component%20Object%20Reference) (OtherBodyIndex :type Integer) (bFromSweep :type Boolean) (SweepResult :type Hit%20Result%20Structure%20%28by%20ref%29))
  (bind _asstatic_mesh_component (Utilities|Casting|CastToStaticMeshComponent OtherComp))
  (Variables|/Game/Keran/BP/MapTactique/BP_StateButton.BP_StateButton_C|SetCamp (Variables|Default|GetStateButtons) _asstatic_mesh_component)
  (Development|PrintString "collision enter"))

(event OnComponentEndOverlap(Capsule)
  (params (OverlappedComponent :type Primitive%20Component%20Object%20Reference) (OtherActor :type Actor%20Object%20Reference) (OtherComp :type Primitive%20Component%20Object%20Reference) (OtherBodyIndex :type Integer))
  (Utilities|Casting|CastToStaticMeshComponent OtherComp)
  (Variables|/Game/Keran/BP/MapTactique/BP_StateButton.BP_StateButton_C|SetCamp (Variables|Default|GetStateButtons) 0)
  (Development|PrintString "collision exit"))

(event EventBeginPlay
  (Variables|/Game/Keran/BP/MapTactique/BP_StateButton.BP_StateButton_C|SetStartRaycast (Variables|Default|GetStateButtons) (Transformation|GetWorldLocation (Variables|Default|GetRaycastStart)))
  (Variables|/Game/Keran/BP/MapTactique/BP_StateButton.BP_StateButton_C|SetEndRaycast (Variables|Default|GetStateButtons) (Transformation|GetWorldLocation (Variables|Default|GetRaycastEnd)))
  (Development|PrintString "Set Raycast Position"))

(event Collision|EventActorBeginOverlap
  (params (OtherActor :type Actor%20Object%20Reference)))

(event EventTick
  (params (DeltaSeconds :type Float%20%28single-precision%29)))

(fn ConstructionScript)