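; BP_MapTacticsSave is an interactive tactics map panel for marking camps as safe, attack or destroy.
; Capsule overlaps set or clear the selected camp mesh, and Interact swaps its material according to the named button.
; Interact returns true only for the map mesh, and MapRotation turns that map by the 2D position delta, returning the current position.
; BeginPlay starts SMCamp green, and debug prints trace overlaps and button presses.
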(event OnComponentBeginOverlap(Capsule)
  (params (OverlappedComponent :type Primitive%20Component%20Object%20Reference) (OtherActor :type Actor%20Object%20Reference) (OtherComp :type Primitive%20Component%20Object%20Reference) (OtherBodyIndex :type Integer) (bFromSweep :type Boolean) (SweepResult :type Hit%20Result%20Structure%20%28by%20ref%29))
  (bind _asstatic_mesh_component (Utilities|Casting|CastToStaticMeshComponent OtherComp))
  (Variables|Map|SetCampSelected _asstatic_mesh_component)
  (Development|PrintString "collision enter"))

(event OnComponentEndOverlap(Capsule)
  (params (OverlappedComponent :type Primitive%20Component%20Object%20Reference) (OtherActor :type Actor%20Object%20Reference) (OtherComp :type Primitive%20Component%20Object%20Reference) (OtherBodyIndex :type Integer))
  (Utilities|Casting|CastToStaticMeshComponent OtherComp)
  (Variables|Map|SetCampSelected 0)
  (Development|PrintString "collision exit"))

(event EventBeginPlay
  (Utilities|FlowControl|Sequence
    (:then_0
      (Rendering|Material|SetMaterial (Variables|Map|GetSM_Camp) 0 "/Game/Keran/Assets/Materials/M_Green.M_Green"))))

(event Collision|EventActorBeginOverlap
  (params (OtherActor :type Actor%20Object%20Reference)))

(event EventTick
  (params (DeltaSeconds :type Float%20%28single-precision%29)))

(fn ConstructionScript)

(fn Interact
  (params (ButtonName :type String))
  (bind _output_get (LocalVariables|SetName ButtonName))
  (switch string _output_get
    (:SM_SafeButton
      (bind _campselected (Variables|Map|GetCampSelected)
        (:then
          (Rendering|Material|SetMaterial _campselected 0 (Variables|StateButton|GetM_Safe))
          (Development|PrintString "Button Safe"))
        (:else
          _)))
    (:SM_AtkButton
      (bind _campselected_2 (Variables|Map|GetCampSelected)
        (:then
          (Rendering|Material|SetMaterial (Variables|Map|GetCampSelected) 0 (Variables|StateButton|GetM_ATK))
          (Development|PrintString "Button ATK"))
        (:else
          _)))
    (:SM_DestroyButton
      (bind _campselected_3 (Variables|Map|GetCampSelected)
        (:then
          (Rendering|Material|SetMaterial (Variables|Map|GetCampSelected) 0 (Variables|StateButton|GetM_Destroy))
          (Development|PrintString "Button Destroy"))
        (:else
          _)))
    (:SM_Map
      (return true))
    (:SM_Base
      (return false)))
  (return false))

(fn MapRotation
  (params (StartPosition :type Vector%202D%20Structure) (ActualPosition :type Vector%202D%20Structure))
  (Transformation|AddWorldRotation (Variables|Map|GetSM_Map) (Math|Rotator|MakeRotator 0.0 (- (.y StartPosition) (.y ActualPosition)) (- (.x StartPosition) (.x ActualPosition))) false false)
  (return (Math|Vector2D|MakeVector2D (.x ActualPosition) (.y ActualPosition))))