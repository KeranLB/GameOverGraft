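; BP_MapTactics is a tactics panel with a touch-rotatable map and Safe, Attack and Destroy buttons for marking camps.
; A capsule overlap selects the camp under aim, and pressing a button swaps that camp's material.
; Dragging rotates SMMap by the touch delta, while a looping timeline samples the drag position.
; Release compares the recent delta to a threshold and plays a reversed timeline that applies inertial spin to SMMapProto.
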(event OnComponentBeginOverlap(Capsule)
  (params (OverlappedComponent :type Primitive%20Component%20Object%20Reference) (OtherActor :type Actor%20Object%20Reference) (OtherComp :type Primitive%20Component%20Object%20Reference) (OtherBodyIndex :type Integer) (bFromSweep :type Boolean) (SweepResult :type Hit%20Result%20Structure%20%28by%20ref%29))
  ;[0.15 0.15 0.15 0.5] Aim Camp Manager
  (bind _asstatic_mesh_component (Utilities|Casting|CastToStaticMeshComponent OtherComp))
  (Variables|Map|SetCampSelected _asstatic_mesh_component))

(event OnComponentEndOverlap(Capsule)
  (params (OverlappedComponent :type Primitive%20Component%20Object%20Reference) (OtherActor :type Actor%20Object%20Reference) (OtherComp :type Primitive%20Component%20Object%20Reference) (OtherBodyIndex :type Integer))
  ;[0.15 0.15 0.15 0.5] Aim Camp Manager
  (Utilities|Casting|CastToStaticMeshComponent OtherComp)
  (Variables|Map|SetCampSelected 0))

(event EventBeginPlay
  ;[0.15 0.15 0.15 0.5] Begin Play
  (Components|Timeline|SetPlayRate (Variables|Default|GetMapRotationInertia) (/ 1.0 (Variables|Inertia|GetInertiaDuration)))
  (Components|Timeline|SetPlayRate (Variables|Default|GetDelayDeltaPosition) (/ 1.0 (Variables|Touch|GetDurationDelayDeltaLocation))))

(event Collision|EventActorBeginOverlap
  (params (OtherActor :type Actor%20Object%20Reference)))

(event EventTick
  (params (DeltaSeconds :type Float%20%28single-precision%29)))

(fn ConstructionScript)

(fn MapRotationFollow
  (params (ActualPosition :type Vector%202D%20Structure))
  (bind _maprotationspeed (Variables|Map|GetMapRotationSpeed))
  (Variables|Touch|SetActualPosition ActualPosition)
  (Variables|Map|GetMapRotation
    (:then
      (Transformation|AddWorldRotation (Variables|Default|GetSM_Map) (Math|Rotator|MakeRotator 0.0 (* _maprotationspeed (- (.y (Variables|Touch|GetStartPosition)) (.y (Variables|Touch|GetActualPosition)))) (* (- (.x (Variables|Touch|GetStartPosition)) (.x (Variables|Touch|GetActualPosition))) _maprotationspeed)) false false)
      (Variables|Touch|SetStartPosition (Variables|Touch|GetActualPosition)))
    (:else)))

(fn MapTacticPressed
  (params (HitComponent :type Primitive%20Component%20Object%20Reference) (StartPosition :type Vector%202D%20Structure))
  (Utilities|FlowControl|Sequence
    (:then_0
      (switch string (Utilities|GetObjectName HitComponent)
        (:SM_SafeButton
          (bind _campselected (Variables|Map|GetCampSelected)
            (:then
              (Rendering|Material|SetMaterial _campselected 0 (Variables|StateButton|GetM_Safe))
              (Development|PrintString "Button Safe"))
            (:else
              _))
          (Variables|Map|SetMapRotation false :!label _label))
        (:SM_AtkButton
          (bind _campselected_2 (Variables|Map|GetCampSelected)
            (:then
              (Rendering|Material|SetMaterial (Variables|Map|GetCampSelected) 0 (Variables|StateButton|GetM_ATK))
              (Development|PrintString "Button ATK")
              (goto _label))
            (:else
              (goto _label))))
        (:SM_DestroyButton
          (bind _campselected_3 (Variables|Map|GetCampSelected)
            (:then
              (Rendering|Material|SetMaterial (Variables|Map|GetCampSelected) 0 (Variables|StateButton|GetM_Destroy))
              (Development|PrintString "Button Destroy")
              (goto _label))
            (:else
              (goto _label))))
        (:SM_Map
          (Variables|Map|SetMapRotation true))))
    (:then_1
      (Variables|Touch|SetStartPosition StartPosition))
    (:then_2
      (Variables|Map|GetMapRotation
        (:then
          (Variables|Inertia|SetInertiaDeltaPosition (Variables|Touch|GetStartPosition))
          (Components|Timeline|PlayfromStart (Variables|Default|GetDelayDeltaPosition))
          (Audio|Components|Audio|Stop (Variables|Default|GetMapRotationInertia)))
        (:else)))))

(fn MapTacticReleased
  (params (ActualTouchPosition :type Vector%202D%20Structure))
  (bind _inertiatreshold (Variables|Inertia|GetInertiaTreshold))
  (Variables|Touch|SetActualPosition ActualTouchPosition)
  (Variables|Map|GetMapRotation
    (:then
      (bind _output_get (Variables|Inertia|SetInertiaDirection (/ (- (Variables|Inertia|GetInertiaDeltaPosition) (Variables|Touch|GetActualPosition)) (Variables|Inertia|GetInertiaDiminutionSpeed))))
      (Development|PrintString (Utilities|String|ToString(Vector2d) _output_get))
      (if (Math|Boolean|ORBoolean (>= (.x (Variables|Inertia|GetInertiaDirection)) (.x _inertiatreshold)) (<= (.x (Variables|Inertia|GetInertiaDirection)) (* -1.0 (.x _inertiatreshold))) (>= (.y (Variables|Inertia|GetInertiaDirection)) (.y _inertiatreshold)) (<= (.y (Variables|Inertia|GetInertiaDirection)) (* -1.0 (.y _inertiatreshold))))
        (Components|Timeline|ReversefromEnd (Variables|Default|GetMapRotationInertia)))
      (Variables|Map|SetMapRotation false))
    (:else)))