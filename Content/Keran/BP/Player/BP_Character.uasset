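; BP_Character is a player character that creates its HUD and can switch between first-person and third-person cameras.
; On BeginPlay it deactivates the third-person camera, then creates WBP_UI_Player, adds it to the viewport and passes itself to the widget as Character.
; The ChangeView event uses the Switch boolean to toggle which of Camera1stView and Camera3dView is active.
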(event Custom|ChangeView
  (if (Variables|Default|GetSwitch)
    (Components|Activation|SetActive (Variables|Default|GetCamera1stView) true false)
    (Components|Activation|SetActive (Variables|Default|GetCamera3dView) false false)
    (Variables|Default|SetSwitch false)
    (else
      (Components|Activation|SetActive (Variables|Default|GetCamera3dView) true false)
      (Components|Activation|SetActive (Variables|Default|GetCamera1stView) false false)
      (Variables|Default|SetSwitch true))))

(event EventBeginPlay
  (Components|Activation|SetActive (Variables|Default|GetCamera3dView) false false)
  (bind _returnvalue (UserInterface|CreateWidget "/Game/Keran/BP/UI/WBP_UI_Player.WBP_UI_Player_C"))
  (bind _output_get (Variables|Default|SetWidgetUI _returnvalue))
  (UserInterface|Viewport|AddtoViewport _output_get 0)
  (Variables|/Game/Keran/BP/UI/WBP_UI_Player.WBP_UI_Player_C|SetCharacter (Variables|Default|GetWidgetUI) self))

(event Collision|EventActorBeginOverlap
  (params (OtherActor :type Actor%20Object%20Reference)))

(event EventTick
  (params (DeltaSeconds :type Float%20%28single-precision%29)))

(fn ConstructionScript)