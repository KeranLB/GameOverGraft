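; Touch player controller that routes gestures to either tactical map manipulation or camera rotation.
; On press, a trace under the cursor checks the hit component's first tag to select the mode stored in EnumAction.
; Map Tactic forwards press, move and release to BP_MapTactics.
; Otherwise, horizontal swipes past a threshold rotate BP_Character_M's camera once per touch, alongside a timeline intended as a swipe time limit.
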(event EventBeginPlay
  ;[0.15 0.15 0.15 0.5] Set Begin Play
  (Components|Timeline|SetPlayRate (Variables|Default|GetDelaySwipeRotationCamera) (/ 1.0 (Variables|RotationCamera|GetDelayStopSwipeRotCam))))

(event Input|TouchEvents|InputTouch
  (params (Location :type Vector) (FingerIndex :type ETouchIndex%20Enum))
  (bind _hitresult (Game|Player|GetHitResultUnderCursorbyChannel "TraceTypeQuery1" true))
  ;[0.15 0.15 0.15 0.5] Touch Manager
  (:Pressed
    (Variables|TouchPressed|SetStartTouchPosition (Math|Vector2D|MakeVector2D (.x Location) (.y Location)))
    (bind _output_get (Variables|TouchPressed|SetHitComponent (.hitcomponent _hitresult)))
    (Variables|TouchPressed|SetHitActor (.hitactor _hitresult))
    (CallFunction|VerifCastActor _output_get))
  (:Released
    (switch Utilities|FlowControl|Switch|SwitchonE_Actor (Variables|TouchPressed|GetEnumAction)
      (:NewEnumerator0
        (Default|MapTacticReleased (Variables|MapTacticPanel|GetMapTactics) (Variables|TouchPressed|GetCurrentTouchPosition)))
      (:NewEnumerator3
        (Variables|TouchPressed|SetIsTouchActive false))))
  (:Moved
    (Variables|TouchPressed|SetCurrentTouchPosition (Math|Vector2D|MakeVector2D (.x Location) (.y Location)))
    (switch Utilities|FlowControl|Switch|SwitchonE_Actor (Variables|TouchPressed|GetEnumAction)
      (:NewEnumerator0
        (Default|MapRotationFollow (Variables|MapTacticPanel|GetMapTactics) (Variables|TouchPressed|GetCurrentTouchPosition)))
      (:NewEnumerator3
        (RotationCamera|CameraRotationMove)))))

(fn ConstructionScript)

(fn CameraRotationPressed
  (Variables|RotationCamera|SetFirstPointerLocation (.x (Variables|TouchPressed|GetStartTouchPosition)))
  (Variables|TouchPressed|SetIsTouchActive true)
  ;[0.15 0.15 0.15 0.5] Makes sure it's a swipe (cancels itself on drag)
  (Components|Timeline|PlayfromStart (Variables|Default|GetDelaySwipeRotationCamera)))

(fn CameraRotationMove
  (bind _output_get (Variables|RotationCamera|SetCurrentPointerLocation (.x (Variables|TouchPressed|GetCurrentTouchPosition))))
  (if (Variables|TouchPressed|GetIsTouchActive)
    (Utilities|FlowControl|Sequence
      (:then_0
        (if (> (- (Variables|RotationCamera|GetFirstPointerLocation) _output_get) (Variables|RotationCamera|GetMovementTreshold))
          (bind _asbp_character_m (Utilities|Casting|CastToBP_Character_M (Game|Player|GetPlayerPawn 0)))
          (Default|RotateCameratoRight _asbp_character_m)
          (Variables|TouchPressed|SetIsTouchActive false)))
      (:then_1
        (if (< (- (Variables|RotationCamera|GetFirstPointerLocation) _output_get) (* -1.0 (Variables|RotationCamera|GetMovementTreshold)))
          (bind _asbp_character_m_2 (Utilities|Casting|CastToBP_Character_M (Game|Player|GetPlayerPawn 0)))
          (Default|RotateCameratoLeft _asbp_character_m_2)
          (Variables|TouchPressed|SetIsTouchActive false))))))

(fn VerifCastActor
  (params (HitComponent :type Primitive%20Component%20Object%20Reference))
  (bind _output_get (LocalVariables|SetComponentHit HitComponent))
  (switch name (Utilities|Array|Get(acopy) (Variables|/Script/Engine.ActorComponent|GetComponentTags _output_get))
    (:Default
      (RotationCamera|CameraRotationPressed)
      (Variables|TouchPressed|SetEnumAction "NewEnumerator3")
      (Development|PrintString "Can Swipe"))
    (:MapTactic
      (bind _asbp_map_tactics (Utilities|Casting|CastToBP_MapTactics (Variables|TouchPressed|GetHitActor)))
      (bind _output_get_2 (Variables|MapTacticPanel|SetMapTactics _asbp_map_tactics))
      (Default|MapTacticPressed _output_get_2 (LocalVariables|GetComponentHit) (Variables|TouchPressed|GetStartTouchPosition))
      (Variables|TouchPressed|SetEnumAction "NewEnumerator0")
      (Development|PrintString "MapTactic"))))