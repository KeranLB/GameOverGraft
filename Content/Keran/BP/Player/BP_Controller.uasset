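; Player controller that shows the mouse cursor and handles touch interaction with the tactics map panel.
; On press, it traces under the cursor for a BP_MapTactics actor and passes the hit component's name to Interact, whose result sets a Follow state.
; While following, touch movement feeds MapRotationFollow, which returns the next start position for incremental dragging, and release clears Follow.
; The hit component name is also printed as debug output.
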(event EventBeginPlay
  (Variables|Default|SetbShowMouseCursor true)
  (Variables|Default|SetPlayerCharacter 0))

(event EventTick
  (params (DeltaSeconds :type Float%20%28single-precision%29)))

(event Input|TouchEvents|InputTouch
  (params (Location :type Vector) (FingerIndex :type ETouchIndex%20Enum))
  (bind _hitresult (Game|Player|GetHitResultUnderCursorbyChannel "TraceTypeQuery1" true))
  (bind _returnvalue (Utilities|GetObjectName (.hitcomponent _hitresult)))
  ;[0.15 0.15 0.15 0.5] Map Tactic Panel
  (:Pressed
    (Variables|MapTacticPanel|SetStartTouchPosition (Math|Vector2D|MakeVector2D (.x Location) (.y Location)))
    (bind _asbp_map_tactics (Utilities|Casting|CastToBP_MapTactics (.hitactor _hitresult)))
    (bind _output_get (Variables|MapTacticPanel|SetMapTactics _asbp_map_tactics))
    (Development|PrintString _returnvalue)
    (bind _maprotation (Default|Interact _output_get _returnvalue))
    (Variables|MapTacticPanel|Setfollow _maprotation))
  (:Released
    (Variables|MapTacticPanel|Setfollow false))
  (:Moved
    (Variables|MapTacticPanel|Getfollow
      (:then
        (bind _newstartposition (Default|MapRotationFollow (Variables|MapTacticPanel|GetMapTactics) (Math|Vector2D|MakeVector2D (.x Location) (.y Location)) (Variables|MapTacticPanel|GetStartTouchPosition)))
        (Variables|MapTacticPanel|SetStartTouchPosition _newstartposition))
      (:else))))

(fn ConstructionScript)