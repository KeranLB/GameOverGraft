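; Player character Blueprint that switches between third-person and first-person cameras and creates the player UI widget.
; The switch is masked by a blink: a timeline closes two UI slider bars, swaps the active camera, then reverses to reopen and hide them.
; In first person, the camera yaws in timeline-lerped steps across three positions, with a camera shake when a turn ends or hits a limit.
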(event Custom|ChangeView
  ;[0.15 0.15 0.15 0.5] 1ST/3RD Swap
  (if (Variables|Default|GetIsInFirstPerson)
    (Components|Activation|SetActive (Variables|Default|GetCamera3dView) true false)
    (Components|Activation|SetActive (Variables|Default|GetCamera1stView) false false)
    (Variables|Default|SetIsInFirstPerson false)
    (else
      (Components|Activation|SetActive (Variables|Default|GetCamera1stView) true false)
      (Components|Activation|SetActive (Variables|Default|GetCamera3dView) false false)
      (Variables|Default|SetIsInFirstPerson true)))
  (Components|Timeline|ReversefromEnd (Variables|Default|GetTimeline_0)))

(event Custom|RotateCameraToLeft
  ;[0.15 0.15 0.15 0.5] 1ST Person Camera Movement
  (if (Variables|Default|GetIsInFirstPerson)
    (if (> (Variables|Default|GetCameraPosition) 0)
      (CallFunction|LerpCamera -45.0)
      (Variables|Default|SetCameraPosition (- (Variables|Default|GetCameraPosition) 1))
      (else
        (bind _asbp_controller_m (Utilities|Casting|CastToBP_Controller_M (Pawn|GetController)))
        (Game|Feedback|ClientStartCameraShake _asbp_controller_m "/Game/Mickael/Blueprints/CamShake_FirstPersonRotation.CamShake_FirstPersonRotation_C" 1.0 "CameraLocal" "0, 0, 0")))))

(event Custom|RotateCameraToRight
  ;[0.15 0.15 0.15 0.5] 1ST Person Camera Movement
  (if (Variables|Default|GetIsInFirstPerson)
    (if (< (Variables|Default|GetCameraPosition) 2)
      (CallFunction|LerpCamera 45.0)
      (Variables|Default|SetCameraPosition (+ (Variables|Default|GetCameraPosition) 1))
      (else
        (bind _asbp_controller_m (Utilities|Casting|CastToBP_Controller_M (Pawn|GetController)))
        (Game|Feedback|ClientStartCameraShake _asbp_controller_m "/Game/Mickael/Blueprints/CamShake_FirstPersonRotation.CamShake_FirstPersonRotation_C" 1.0 "CameraLocal" "0, 0, 0")))))

(event Custom|LerpCamera
  (params (B%20Z%20%28Yaw%29 :type Float%20%28single-precision%29))
  (bind _camera1stview (Variables|Default|GetCamera1stView))
  (bind _returnvalue (Transformation|GetWorldRotation _camera1stview))
  ;[0.15 0.15 0.15 0.5] 1ST Person Camera Movement
  (Variables|Default|SetStartRotation (Math|Vector|MakeVector (.roll _returnvalue) (.pitch _returnvalue) (.yaw _returnvalue)))
  (bind _newtrack_0 (Timeline|CameraRotation PlayFromStart)
    (:Update
      (Transformation|SetWorldRotation (Variables|Default|GetCamera1stView) (Math|Rotator|MakeRotator 0.0 0.0 (Math|Float|Lerp (.z (Variables|Default|GetStartRotation)) (+ (.z (Variables|Default|GetStartRotation)) B%20Z%20%28Yaw%29) _newtrack_0)) false false))
    (:Finished
      (bind _asbp_controller_m (Utilities|Casting|CastToBP_Controller_M (Pawn|GetController)))
      (Game|Feedback|ClientStartCameraShake _asbp_controller_m "/Game/Mickael/Blueprints/CamShake_FirstPersonRotation.CamShake_FirstPersonRotation_C" 1.0 "CameraLocal" "0, 0, 0"))))

(event Custom|BlinkIN
  ;[0.15 0.15 0.15 0.5] 1ST/3RD Swap
  (Widget|SetVisibility (Variables|/Game/Mickael/Blueprints/WBP_UI_Player_M.WBP_UI_Player_M_C|GetBottomSlider (Variables|Default|GetWidgetUI)) "Visible")
  (Widget|SetVisibility (Variables|/Game/Mickael/Blueprints/WBP_UI_Player_M.WBP_UI_Player_M_C|GetTopSlider (Variables|Default|GetWidgetUI)) "Visible")
  (Variables|Default|SetIsBlinking true)
  (bind _blinkin (Timeline|Timeline_0 PlayFromStart)
    (:Update
      (Progress|SetPercent (Variables|/Game/Mickael/Blueprints/WBP_UI_Player_M.WBP_UI_Player_M_C|GetTopSlider (Variables|Default|GetWidgetUI)) _blinkin)
      (Progress|SetPercent (Variables|/Game/Mickael/Blueprints/WBP_UI_Player_M.WBP_UI_Player_M_C|GetBottomSlider (Variables|Default|GetWidgetUI)) _blinkin))
    (:Finished
      (if (Variables|Default|GetIsBlinking)
        (Variables|Default|SetIsBlinking false)
        (CallFunction|ChangeView)
        (else
          (Widget|SetVisibility (Variables|/Game/Mickael/Blueprints/WBP_UI_Player_M.WBP_UI_Player_M_C|GetBottomSlider (Variables|Default|GetWidgetUI)) "Hidden")
          (Widget|SetVisibility (Variables|/Game/Mickael/Blueprints/WBP_UI_Player_M.WBP_UI_Player_M_C|GetTopSlider (Variables|Default|GetWidgetUI)) "Hidden"))))))

(event EventBeginPlay
  (Utilities|FlowControl|Sequence
    (:then_0
      ;[0.15 0.15 0.15 0.5] UI Player
      (Components|Activation|SetActive (Variables|Default|GetCamera3dView) true false)
      (bind _returnvalue (UserInterface|CreateWidget "/Game/Mickael/Blueprints/WBP_UI_Player_M.WBP_UI_Player_M_C"))
      (bind _output_get (Variables|Default|SetWidgetUI _returnvalue))
      (UserInterface|Viewport|AddtoViewport _output_get 0)
      (Variables|/Game/Mickael/Blueprints/WBP_UI_Player_M.WBP_UI_Player_M_C|SetCharacter (Variables|Default|GetWidgetUI) self))
    (:then_1
      ;[0.15 0.15 0.15 0.5] Camera Rotation Speed
      (Components|Timeline|SetPlayRate (Variables|Default|GetCameraRotation) (/ 1.0 (Variables|Default|GetRotationSpeed)))
      ;[0.15 0.15 0.15 0.5] Blink Speed
      (Components|Timeline|SetPlayRate (Variables|Default|GetTimeline_0) (/ 1.0 (Variables|Default|GetBlinkSpeed))))))

(fn ConstructionScript)