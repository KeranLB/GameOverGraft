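; BP_Gauge is a timed gauge that drives a WBP_Gauge widget's green-to-red gradient and the enemy's state.
; One Timeline feeds the widget, passes stage changes to the enemy, and on finishing either restarts or, given a valid main gauge, ends the game.
; Task success briefly reverses the Timeline to add time, while failure briefly speeds it up to subtract time.
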(event Custom|TaskSucceed
  (params (TimeToAdd :type Float%20%28double-precision%29))
  (Utilities|String|Reverse (Variables|Default|GetTimeline))
  (Utilities|FlowControl|Delay TimeToAdd)
  (Audio|Components|Audio|Play (Variables|Default|GetTimeline)))

(event Custom|TaskFailed
  (params (TimeToSubtract :type Float%20%28double-precision%29))
  (Components|Timeline|SetPlayRate (Variables|Default|GetTimeline) (/ 1.0 (Variables|Default|GetGaugeAccelerateSpeed)))
  (Utilities|FlowControl|Delay (/ TimeToSubtract (Variables|AtomicParameters|GetAccelerationParam)))
  (Components|Timeline|SetPlayRate (Variables|Default|GetTimeline) (/ 1.0 (Variables|AtomicParameters|GetGaugeTimeSpeed))))

(event EventBeginPlay
  (bind _timeline (Variables|Default|GetTimeline))
  ;[0.15 0.15 0.15 0.5] Init all the parameters
  (bind _aswbp_gauge (Utilities|Casting|CastToWBP_Gauge (UserInterface|GetWidget (Variables|Default|GetGauge_1))))
  (Variables|Default|SetUIGauge _aswbp_gauge)
  (Components|Timeline|SetPlayRate _timeline (/ 1.0 (Variables|AtomicParameters|GetGaugeTimeSpeed)))
  (Components|Timeline|PlayfromStart _timeline)
  (Variables|Default|SetGaugeAccelerateSpeed (/ (Variables|AtomicParameters|GetGaugeTimeSpeed) (Variables|AtomicParameters|GetAccelerationParam))))

(fn ConstructionScript)