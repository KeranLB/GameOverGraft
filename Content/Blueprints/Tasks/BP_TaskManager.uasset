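; BP_TaskManager spawns and tracks BP_Task actors in fixed position slots, freeing each slot when emptied.
; Each task draws random data from a list chosen by caller (President, Ministre, Commandant, Soldat, Service Medical) and difficulty, removing the entry to avoid duplicates.
; New tasks link to the first free button panel, passing their code count.
; Map panel inputs are matched against started tasks' base and status pairs, advancing a step once all three match.
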(fn ConstructionScript)

(fn SpawnTask
  (params (Caller :type E_Caller%20Enum :default "NewEnumerator0"))
  (bind _returnvalue (Transformation|GetActorTransform))
  (bind (_array_element _array_index) (Utilities|Array|ForEachLoopwithBreak (Variables|Spawning|GetIsPositionTaken))
    (:LoopBody
      ;[0.15 0.15 0.15 0.5] Spawns the task actor in a free position
      (if (not _array_element)
        (bind _returnvalue_2 (Game|SpawnActorfromClass "/Game/Blueprints/Tasks/BP_Task.BP_Task_C" (Math|Transform|MakeTransform (+ (Utilities|Array|Get(acopy) (Variables|Spawning|GetPositions) _array_index) (.location _returnvalue)) (Math|Rotator|MakeRotator (.roll (.rotation _returnvalue)) (.pitch (.rotation _returnvalue)) (- (.yaw (.rotation _returnvalue)) 9e+01)) (.scale _returnvalue)) "Undefined" "MultiplyWithRoot" 0 0))
        ;[0.15 0.15 0.15 0.5] Keeps Tracks of the task
        (bind _output_get (Variables|ProgressTracking|SetOutputTask _returnvalue_2))
        (Utilities|Array|SetArrayElem (Variables|ProgressTracking|GetCurrentTasks) _array_index _output_get)
        ;[0.15 0.15 0.15 0.5] Depending on Caller and Difficulty
        (TaskHandling|ChangeDataListwithCaller Caller)
        ;[0.15 0.15 0.15 0.5] Takes a random index (task data) and removes it from the list. Prevents dupplicates.
        (LocalVariables|SetIndexToRemove (Math|Random|RandomInteger (Utilities|Array|Length (Variables|Spawning|GetDataList))))
        (Default|Initialize _output_get (Utilities|Array|Get(acopy) (Variables|Spawning|GetDataList) (LocalVariables|GetIndexToRemove)) self _array_index)
        (Utilities|Array|RemoveIndex (Variables|Spawning|GetDataList) (LocalVariables|GetIndexToRemove))
        (PanelSpecific|LinkTasktoButtonPanel (Variables|ProgressTracking|GetOutputTask))
        ;[0.15 0.15 0.15 0.5] Marks the slot as unavailable
        (Utilities|Array|SetArrayElem (Variables|Spawning|GetIsPositionTaken) _array_index true)
        (return (Variables|ProgressTracking|GetOutputTask))))))

(fn EmptyTaskSlot
  (params (TaskIndex :type Integer) (ButtonPanelIndex :type Integer))
  ;[0.15 0.15 0.15 0.5] Makes the slot available for new tasks
  (Utilities|Array|SetArrayElem (Variables|Spawning|GetIsPositionTaken) TaskIndex false)
  ;;[0.15 0.15 0.15 0.5] If button panel is involved, clears concerning panel's slot
  (if (== (Utilities|Array|Get(acopy) (Variables|ProgressTracking|GetCurrentTasks) TaskIndex) (Variables|/Game/Blueprints/Panels/BP_ButtonPanel.BP_ButtonPanel_C|GetBP_Task (Utilities|Array|Get(acopy) (Variables|ButtonPanel|GetButtonPanels%20List) ButtonPanelIndex)))
    (Utilities|Array|SetArrayElem (Variables|ButtonPanel|GetButtonPanels%20List) ButtonPanelIndex 0))
  (Utilities|Array|SetArrayElem (Variables|ProgressTracking|GetCurrentTasks) TaskIndex 0))

(fn ChangeDataList
  (params (CallerStructure :type F%20Task%20Difficulty%20Structure%20Structure))
  (switch Utilities|FlowControl|Switch|SwitchonE_DifficultyTask (Variables|DifficultySorting|GetTaskDifficultyEnum)
    (:NewEnumerator0
      (|SetBy-RefVar (Variables|Spawning|GetDataList) (.p1d1 CallerStructure))
      (Development|PrintString "Hello"))
    (:NewEnumerator1
      (|SetBy-RefVar (Variables|Spawning|GetDataList) (.p1d2 CallerStructure)))
    (:NewEnumerator2
      (|SetBy-RefVar (Variables|Spawning|GetDataList) (.p1d3 CallerStructure)))
    (:NewEnumerator3
      (|SetBy-RefVar (Variables|Spawning|GetDataList) (.p2d1 CallerStructure)))
    (:NewEnumerator4
      (|SetBy-RefVar (Variables|Spawning|GetDataList) (.p2d2 CallerStructure)))
    (:NewEnumerator5
      (|SetBy-RefVar (Variables|Spawning|GetDataList) (.p2d3 CallerStructure)))
    (:NewEnumerator6
      (|SetBy-RefVar (Variables|Spawning|GetDataList) (.p3d1 CallerStructure)))
    (:NewEnumerator7
      (|SetBy-RefVar (Variables|Spawning|GetDataList) (.p3d2 CallerStructure)))
    (:NewEnumerator8
      (|SetBy-RefVar (Variables|Spawning|GetDataList) (.p3d3 CallerStructure)))))

(fn LinkTasktoButtonPanel
  (params (Task :type BP%20Task%20Object%20Reference))
  ;[0.15 0.15 0.15 0.5] If no task are found in the button panel, link one
  ;;[0.15 0.15 0.15 0.5] Info to Panel
  (bind (_array_element _array_index) (Utilities|Array|ForEachLoopwithBreak (Variables|ButtonPanel|GetButtonPanels%20List) :!label _label)
    (:LoopBody
      (Utilities|IsValid (Variables|/Game/Blueprints/Panels/BP_ButtonPanel.BP_ButtonPanel_C|GetBP_Task _array_element)
        (:Is%20Not%20Valid
          (bind _output_get (Variables|/Game/Blueprints/Panels/BP_ButtonPanel.BP_ButtonPanel_C|SetBP_Task _array_element Task))
          (Variables|/Game/Blueprints/Panels/BP_ButtonPanel.BP_ButtonPanel_C|SetNbSymbolToGenerate _array_element (Variables|/Game/Blueprints/Tasks/BP_Task.BP_Task_C|GetNumberOfCodes _output_get))
          ;;[0.15 0.15 0.15 0.5] Info to BP Task
          (Variables|/Game/Blueprints/Tasks/BP_Task.BP_Task_C|SetButtonPanelPositionIndex Task _array_index)
          (goto _label Break))))))

(fn MapPanelCheckStep
  (params (Base :type E_BasesNames%20Enum :default "NewEnumerator0") (Status :type E_BasesStatuses%20Enum :default "NewEnumerator0"))
  ;[0.15 0.15 0.15 0.5] Checks every task for a match.
  (for _array_element (Variables|ProgressTracking|GetCurrentTasks)
    (Utilities|IsValid _array_element
      (:Is%20Valid
        ;;[0.15 0.15 0.15 0.5] Prevents grayedout tasks to be checked
        (if (Variables|/Game/Blueprints/Tasks/BP_Task.BP_Task_C|GetHasStarted _array_element)
          (bind (_array_element_2 _array_index) (Utilities|Array|ForEachLoopwithBreak (Variables|/Game/Blueprints/Tasks/BP_Task.BP_Task_C|GetBaseName _array_element))
            (:LoopBody
              (if (and (Utilities|Enum|Equal(Enum) (Utilities|String|EnumtoString _array_element_2) (Utilities|String|EnumtoString Base)) (Utilities|Enum|Equal(Enum) (Utilities|String|EnumtoString (Utilities|Array|Get(acopy) (Variables|/Game/Blueprints/Tasks/BP_Task.BP_Task_C|GetBaseStatus _array_element) _array_index)) (Utilities|String|EnumtoString Status)))
                (Utilities|Array|SetArrayElem (Variables|/Game/Blueprints/Tasks/BP_Task.BP_Task_C|GetBasesCheckList _array_element) _array_index true)
                ;[0.15 0.15 0.15 0.5] If all maps are updated
                (if (and (and (Utilities|Array|Get(acopy) (Variables|/Game/Blueprints/Tasks/BP_Task.BP_Task_C|GetBasesCheckList _array_element)) (Utilities|Array|Get(acopy) (Variables|/Game/Blueprints/Tasks/BP_Task.BP_Task_C|GetBasesCheckList _array_element) 1)) (Utilities|Array|Get(acopy) (Variables|/Game/Blueprints/Tasks/BP_Task.BP_Task_C|GetBasesCheckList _array_element) 2))
                  (Default|CheckStep _array_element 1))
                (return "true"))))))))
  (return false))

(fn ChangeDataListwithCaller
  (params (Caller :type E_Caller%20Enum :default "NewEnumerator0"))
  (bind _callerstructure (Variables|DifficultySorting|GetCallerStructure))
  (switch Utilities|FlowControl|Switch|SwitchonE_Caller Caller
    (:NewEnumerator0
      (TaskHandling|ChangeDataList (.president _callerstructure)))
    (:NewEnumerator1
      (TaskHandling|ChangeDataList (.ministe _callerstructure)))
    (:NewEnumerator2
      (TaskHandling|ChangeDataList (.commandant _callerstructure)))
    (:NewEnumerator3
      (TaskHandling|ChangeDataList (.soldat _callerstructure)))
    (:NewEnumerator4
      (TaskHandling|ChangeDataList (.servicemedical _callerstructure)))))