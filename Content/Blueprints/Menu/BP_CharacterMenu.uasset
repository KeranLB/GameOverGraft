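; Menu pawn that presents a first-person camera rotating between three preset viewpoints, starting on the title screen, and opens the game level on StartGame.
; Rotate left/right events drive a timeline, rate-scaled by RotationSpeed, that lerps the camera between neighboring placeholder transforms and then updates the position index.
; A camera shake plays through BP_ControllerMenu when a rotation finishes or is blocked at either end.
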(event Custom|RotateCameraToLeft
  ;[0.15 0.15 0.15 0.5] 1ST Person Camera Movement
  (if (> (Variables|Camera|GetCameraPosition) 0)
    (CallFunction|LerpCamera -1)
    (else
      (bind _asbp_controller_menu (Utilities|Casting|CastToBP_ControllerMenu (Pawn|GetController)))
      (Game|Feedback|ClientStartCameraShake _asbp_controller_menu "/Game/UI/FirstPersonUI/CamShake_FirstPersonRotation.CamShake_FirstPersonRotation_C" 1.0 "CameraLocal" "0, 0, 0"))))

(event Custom|RotateCameraToRight
  ;[0.15 0.15 0.15 0.5] 1ST Person Camera Movement
  (if (< (Variables|Camera|GetCameraPosition) 2)
    (CallFunction|LerpCamera 1)
    (else
      (bind _asbp_controller_menu (Utilities|Casting|CastToBP_ControllerMenu (Pawn|GetController)))
      (Game|Feedback|ClientStartCameraShake _asbp_controller_menu "/Game/UI/FirstPersonUI/CamShake_FirstPersonRotation.CamShake_FirstPersonRotation_C" 1.0 "CameraLocal" "0, 0, 0"))))

(event Custom|LerpCamera
  (params (TargetTransformIndex :type Integer))
  ;[0.15 0.15 0.15 0.5] 1ST Person Camera Movement
  (bind _newtrack_0 (Timeline|CameraRotation PlayFromStart)
    (:Update
      (Transformation|SetWorldLocationAndRotation (Variables|Camera|GetCamera1stView) (.location (Math|Transform|Lerp(Transform) (Transformation|GetWorldTransform (Utilities|Array|Get(acopy) (Variables|Camera|GetTransformsCam) (Variables|Camera|GetCameraPosition))) (Transformation|GetWorldTransform (Utilities|Array|Get(acopy) (Variables|Camera|GetTransformsCam) (+ TargetTransformIndex (Variables|Camera|GetCameraPosition)))) _newtrack_0)) (.rotation (Math|Transform|Lerp(Transform) (Transformation|GetWorldTransform (Utilities|Array|Get(acopy) (Variables|Camera|GetTransformsCam) (Variables|Camera|GetCameraPosition))) (Transformation|GetWorldTransform (Utilities|Array|Get(acopy) (Variables|Camera|GetTransformsCam) (+ TargetTransformIndex (Variables|Camera|GetCameraPosition)))) _newtrack_0)) false false))
    (:Finished
      (bind _asbp_controller_menu (Utilities|Casting|CastToBP_ControllerMenu (Pawn|GetController)))
      (Game|Feedback|ClientStartCameraShake _asbp_controller_menu "/Game/UI/FirstPersonUI/CamShake_FirstPersonRotation.CamShake_FirstPersonRotation_C" 1.0 "CameraLocal" "0, 0, 0")
      (Variables|Camera|SetCameraPosition (+ (Variables|Camera|GetCameraPosition) TargetTransformIndex)))))

(event Custom|StartGame
  (Game|OpenLevel(byObjectReference) "/Game/Levels/Lvl_Félix_Light.Lvl_Félix_Light"))

(event EventBeginPlay
  (bind _transformscam (Variables|Camera|GetTransformsCam))
  (bind _cameraposition (Variables|Camera|GetCameraPosition))
  (bind _output (Utilities|Array|Get(acopy) _transformscam _cameraposition))
  (bind _returnvalue (Transformation|GetWorldTransform _output))
  ;[0.15 0.15 0.15 0.5] Camera Rotation Speed
  (Components|Timeline|SetPlayRate (Variables|Default|GetCameraRotation) (/ 1.0 (Variables|AtomicParameters|GetRotationSpeed)))
  ;[0.15 0.15 0.15 0.5] Set the 3 positions of the 1st view Camera
  (Utilities|Array|SetArrayElem (Variables|Camera|GetTransformsCam) 0 (Variables|Default|GetEmptyTaget_0))
  (Utilities|Array|SetArrayElem (Variables|Camera|GetTransformsCam) 1 (Variables|Default|GetEmptyTaget_1))
  (Utilities|Array|SetArrayElem (Variables|Camera|GetTransformsCam) 2 (Variables|Components|GetEmptyTaget_2))
  ;[0.15 0.15 0.15 0.5] Set 1st view camera to the Title Screen
  (Transformation|SetWorldLocationAndRotation (Variables|Camera|GetCamera1stView) (.location _returnvalue) (.rotation _returnvalue) false false))

(fn ConstructionScript)