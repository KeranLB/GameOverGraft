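; Menu play screen actor where dragging a cable into a slot starts the game through BP_CharacterMenu.
; CablePressed, CableFollow and CableReleased handle the drag, moving the cable by the scaled pointer delta in local X/Z.
; Box overlaps track whether the slot is occupied and choose the cable's snap pose: seated in the slot or back at its start position.
; Releasing applies that pose and calls StartGame if the slot is occupied.
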(event OnComponentBeginOverlap(Box)
  (params (OverlappedComponent :type Primitive%20Component%20Object%20Reference) (OtherActor :type Actor%20Object%20Reference) (OtherComp :type Primitive%20Component%20Object%20Reference) (OtherBodyIndex :type Integer) (bFromSweep :type Boolean) (SweepResult :type Hit%20Result%20Structure%20%28by%20ref%29))
  (Variables|Cable|SetIsInEmplacement true)
  (if (== OtherComp (Variables|Default|GetSM_Cable_002))
    (Variables|Cable|SetReleasedPosition (Variables|/Script/Engine.SceneComponent|GetRelativeLocation (Variables|Default|GetBox)))
    (Variables|Cable|SetReleasedRotation "0.000000,180.000000,90.000000")))

(event OnComponentEndOverlap(Box)
  (params (OverlappedComponent :type Primitive%20Component%20Object%20Reference) (OtherActor :type Actor%20Object%20Reference) (OtherComp :type Primitive%20Component%20Object%20Reference) (OtherBodyIndex :type Integer))
  (Variables|Cable|SetIsInEmplacement false)
  (if (== OtherComp (Variables|Default|GetSM_Cable_002))
    (Variables|Cable|SetReleasedPosition (Variables|Cable|GetStartPositionCable))
    (Variables|Cable|SetReleasedRotation "0.000000,180.000000,-20.000000")))

(event Custom|StartGame
  (Default|StartGame (Variables|Default|GetPlayer)))

(event EventBeginPlay
  (bind _output_get (Variables|Cable|SetStartPositionCable (Variables|/Script/Engine.SceneComponent|GetRelativeLocation (Variables|Default|GetSM_Cable_002))))
  (Variables|Cable|SetReleasedPosition _output_get)
  (bind _asbp_character_menu (Utilities|Casting|CastToBP_CharacterMenu (Game|GetPlayerCharacter 0)))
  (Variables|Default|SetPlayer _asbp_character_menu))

(fn ConstructionScript)

(fn CableFollow
  (params (ActualPosition :type Vector%202D%20Structure))
  (Variables|CableFollow|GetCanCableFollow
    (:then
      (Variables|CableFollow|SetActualPosition ActualPosition)
      (Transformation|AddRelativeLocation (Variables|Default|GetSM_Cable_002) (Math|Vector|MakeVector (.x (* (Math|Vector2D|MakeVector2D (- (.x (Variables|CableFollow|GetActualPosition)) (.x (Variables|CableFollow|GetStartPosition))) (- (.y (Variables|CableFollow|GetStartPosition)) (.y (Variables|CableFollow|GetActualPosition)))) (Variables|CableFollow|GetCableFollowSpeed))) 0.0 (.y (* (Math|Vector2D|MakeVector2D (- (.x (Variables|CableFollow|GetActualPosition)) (.x (Variables|CableFollow|GetStartPosition))) (- (.y (Variables|CableFollow|GetStartPosition)) (.y (Variables|CableFollow|GetActualPosition)))) (Variables|CableFollow|GetCableFollowSpeed)))) false false)
      (Variables|CableFollow|SetStartPosition (Variables|CableFollow|GetActualPosition)))
    (:else)))

(fn CablePressed
  (params (StartPosition :type Vector%202D%20Structure) (HitCompo :type Primitive%20Component%20Object%20Reference))
  (Variables|CableFollow|SetStartPosition StartPosition)
  (switch name (Utilities|Array|Get(acopy) (Variables|/Script/Engine.ActorComponent|GetComponentTags HitCompo))
    (:Cable
      (Variables|CableFollow|SetCanCableFollow true)
      (Transformation|SetRelativeRotation (Variables|Default|GetSM_Cable_002) "0.000000,180.000000,90.000000" false false))))

(fn CableReleased
  (Variables|CableFollow|GetCanCableFollow
    (:then
      (Variables|CableFollow|SetCanCableFollow false)
      (Transformation|SetRelativeLocationAndRotation (Variables|Default|GetSM_Cable_002) (Variables|Cable|GetReleasedPosition) (Variables|Cable|GetReleasedRotation) false false)
      (Variables|Cable|GetIsInEmplacement
        (:then
          (CallFunction|StartGame))
        (:else)))
    (:else)))