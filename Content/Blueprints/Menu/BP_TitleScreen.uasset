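; BP_TitleScreen is a menu Blueprint that toggles its SMTask component between a resting position and one slightly raised on local Z.
; BeginPlay caches both positions and scales the timeline's play rate from OpenCloseMovementSpeed.
; OpenClose plays or reverses OpenCloseTimeline according to IsOpened, with IsOpening as a guard against retriggering mid-move.
; The timeline lerps SMTask's relative location and clears IsOpening when finished.
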(event EventBeginPlay
  (bind _output_get (Variables|Default|SetBaseLocation (Variables|/Script/Engine.SceneComponent|GetRelativeLocation (Variables|Default|GetSM_Task))))
  (Variables|Default|SetTargetLocation (+ _output_get "0.000000,0.000000,32.000000"))
  (Components|Timeline|SetPlayRate (Variables|Default|GetOpenCloseTimeline) (/ 1.0 (Variables|Default|GetOpenCloseMovementSpeed))))

(fn ConstructionScript)

(fn OpenClose
  (Variables|Default|GetIsOpening
    (:then)
    (:else
      (if (Variables|Default|GetIsOpened)
        (Components|Timeline|ReversefromEnd (Variables|Default|GetOpenCloseTimeline))
        (Variables|Default|SetIsOpening true)
        (Variables|Default|SetIsOpened false)
        (else
          (Components|Timeline|PlayfromStart (Variables|Default|GetOpenCloseTimeline))
          (Variables|Default|SetIsOpening true)
          (Variables|Default|SetIsOpened true))))))