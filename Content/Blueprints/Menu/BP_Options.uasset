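; Options menu Blueprint with 3D levers that switch the Posterize and Volume settings stored in BP_GI_test, both forced on at BeginPlay.
; SwitchClicked routes the hit component's first tag to that lever's function, which writes the game instance flag.
; A shared LeverSwitch timeline plays forward or backward to roll the selected lever, with CanSwitch gating clicks during motion.
; Both branches of LeverVolumeSwitch set the flag false, so Volume never turns back on.
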(event EventBeginPlay
  (bind _asbp_gi_test (Utilities|Casting|CastToBP_GI_test (Game|GetGameInstance)))
  (Variables|/Game/Save/BP_GI_test.BP_GI_test_C|SetActivePosterize _asbp_gi_test true)
  (Variables|/Game/Save/BP_GI_test.BP_GI_test_C|SetActiveVolume _asbp_gi_test true)
  (Components|Timeline|SetPlayRate (Variables|Default|GetLeverSwitch) (/ 1.0 (Variables|AtomicParameters|GetLeverSwitchSpeed))))

(fn ConstructionScript)

(fn LeverSposterizeSwitch
  (Variables|animation|GetCanSwitch
    (:then
      (Variables|Posterize|GetLeverPosterize
        (:then
          (bind _output_get (Variables|Posterize|SetLeverPosterize false))
          (bind _asbp_gi_test (Utilities|Casting|CastToBP_GI_test (Game|GetGameInstance)))
          (Variables|/Game/Save/BP_GI_test.BP_GI_test_C|SetActivePosterize _asbp_gi_test _output_get)
          (Variables|animation|SetCanSwitch false)
          (Variables|Animation|SetLeverSwitching (Variables|Posterize|GetSM_Posterize_Lever))
          (Components|Timeline|PlayfromStart (Variables|Default|GetLeverSwitch)))
        (:else
          (bind _output_get_2 (Variables|Posterize|SetLeverPosterize true))
          (bind _asbp_gi_test_2 (Utilities|Casting|CastToBP_GI_test (Game|GetGameInstance)))
          (Variables|/Game/Save/BP_GI_test.BP_GI_test_C|SetActivePosterize _asbp_gi_test_2 _output_get_2)
          (Variables|animation|SetCanSwitch false)
          (Variables|Animation|SetLeverSwitching (Variables|Posterize|GetSM_Posterize_Lever))
          (Components|Timeline|ReversefromEnd (Variables|Default|GetLeverSwitch)))))
    (:else)))

(fn LeverVolumeSwitch
  (Variables|animation|GetCanSwitch
    (:then
      (Variables|Volume|GetLeverVolume
        (:then
          (bind _output_get (Variables|Volume|SetLeverVolume false))
          (bind _asbp_gi_test (Utilities|Casting|CastToBP_GI_test (Game|GetGameInstance)))
          (Variables|/Game/Save/BP_GI_test.BP_GI_test_C|SetActiveVolume _asbp_gi_test _output_get)
          (Variables|animation|SetCanSwitch false)
          (Variables|Animation|SetLeverSwitching (Variables|Volume|GetSM_Volume_Lever))
          (Components|Timeline|PlayfromStart (Variables|Default|GetLeverSwitch)))
        (:else
          (bind _output_get_2 (Variables|Volume|SetLeverVolume false))
          (bind _asbp_gi_test_2 (Utilities|Casting|CastToBP_GI_test (Game|GetGameInstance)))
          (Variables|/Game/Save/BP_GI_test.BP_GI_test_C|SetActiveVolume _asbp_gi_test_2 _output_get_2)
          (Variables|animation|SetCanSwitch false)
          (Variables|Animation|SetLeverSwitching (Variables|Volume|GetSM_Volume_Lever))
          (Components|Timeline|ReversefromEnd (Variables|Default|GetLeverSwitch)))))
    (:else)))

(fn SwitchClicked
  (params (ComponentHit :type Primitive%20Component%20Object%20Reference))
  (bind _componenttags (Variables|/Script/Engine.ActorComponent|GetComponentTags ComponentHit))
  (bind _output (Utilities|Array|Get(acopy) _componenttags))
  (Development|PrintString (Utilities|String|ToString(Name) _output))
  (switch name _output
    (:Posterize
      (CallFunction|LeverSposterizeSwitch))
    (:Volume
      (CallFunction|LeverVolumeSwitch))))