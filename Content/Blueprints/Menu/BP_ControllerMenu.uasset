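; Player controller for the menu that routes single-finger touches to interactive 3D menu actors or to camera rotation.
; On press, a trace under the finger reads the hit actor's first tag to target the options panel, play screen cable or title screen credits.
; Other touches become horizontal swipes that rotate the menu character's camera left or right past a threshold, with a timeline meant to limit swipe duration.
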(event EventBeginPlay
  ;[0.15 0.15 0.15 0.5] Set Begin Play
  (Components|Timeline|SetPlayRate (Variables|Default|GetDelaySwipeRotationCamera) (/ 1.0 (Variables|RotationCamera|GetDelayStopSwipeRotCam)))
  (bind _asbp_character_menu (Utilities|Casting|CastToBP_CharacterMenu (Game|Player|GetPlayerPawn 0)))
  (Variables|Default|SetPlayerCharacter _asbp_character_menu))

(event Input|TouchEvents|InputTouch
  (params (Location :type Vector) (FingerIndex :type ETouchIndex%20Enum))
  (bind _hitresult (Class|PlayerController|GetHitResultUnderFingerbyChannel "Touch1" "TraceTypeQuery1" true))
  ;[0.15 0.15 0.15 0.5] Touch Manager
  (:Pressed
    (switch Utilities|FlowControl|Switch|SwitchonETouchIndex FingerIndex
      (:Touch1
        ;;[0.15 0.15 0.15 0.5] Pressed
        (Variables|TouchPressed|SetStartTouchPosition (Math|Vector2D|MakeVector2D (.x Location) (.y Location)))
        (Variables|Default|SetHitComponent (.hitcomponent _hitresult))
        (Variables|TouchPressed|SetHitActor (.hitactor _hitresult))
        (CallFunction|VerifCastActor)
        (switch Utilities|FlowControl|Switch|SwitchonE_MenuPanels (Variables|CastActor|GetEnumActor)
          (:NewEnumerator1
            (Default|SwitchClicked (Variables|CastActor|GetOptionPanel) (Variables|Default|GetHitComponent)))
          (:NewEnumerator2
            (Default|CablePressed (Variables|CastActor|GetPlayScreen) (Variables|TouchPressed|GetStartTouchPosition) (Variables|Default|GetHitComponent)))
          (:NewEnumerator3
            ;;;[0.15 0.15 0.15 0.5] Credits
            (Default|OpenClose (Variables|CastActor|GetCredits)))))))
  (:Released
    (switch Utilities|FlowControl|Switch|SwitchonETouchIndex FingerIndex
      (:Touch1
        ;;[0.15 0.15 0.15 0.5] Released
        (switch Utilities|FlowControl|Switch|SwitchonE_MenuPanels (Variables|CastActor|GetEnumActor)
          (:NewEnumerator2
            (Default|CableReleased (Variables|CastActor|GetPlayScreen)))
          (:NewEnumerator4
            (Variables|TouchPressed|SetIsTouchActive false))))))
  (:Moved
    (switch Utilities|FlowControl|Switch|SwitchonETouchIndex FingerIndex
      (:Touch1
        ;;[0.15 0.15 0.15 0.5] Move
        (Variables|TouchPressed|SetCurrentTouchPosition (Math|Vector2D|MakeVector2D (.x Location) (.y Location)))
        (switch Utilities|FlowControl|Switch|SwitchonE_MenuPanels (Variables|CastActor|GetEnumActor)
          (:NewEnumerator2
            (Default|CableFollow (Variables|CastActor|GetPlayScreen) (Variables|TouchPressed|GetCurrentTouchPosition)))
          (:NewEnumerator4
            (RotationCamera|CameraRotationMove)))))))

(fn ConstructionScript)

(fn VerifCastActor
  (bind _hitactor (Variables|TouchPressed|GetHitActor))
  (bind _tags (Variables|/Script/Engine.Actor|GetTags _hitactor))
  (Utilities|IsValid _hitactor
    (:Is%20Valid
      (if (Utilities|Array|IsValidIndex _tags)
        (switch name (Utilities|Array|Get(acopy) _tags)
          (:Default
            ;[0.15 0.15 0.15 0.5] Camera Rotation
            (RotationCamera|CameraRotationPressed :!label _label)
            (Variables|CastActor|SetEnumActor "NewEnumerator4"))
          (:Option
            (bind _asbp_options (Utilities|Casting|CastToBP_Options (Variables|TouchPressed|GetHitActor)))
            (Variables|CastActor|SetOptionPanel _asbp_options)
            (Variables|CastActor|SetEnumActor "NewEnumerator1"))
          (:Play
            (bind _asbp_play_screen (Utilities|Casting|CastToBP_PlayScreen (Variables|TouchPressed|GetHitActor)))
            (Variables|CastActor|SetPlayScreen _asbp_play_screen)
            (Variables|CastActor|SetEnumActor "NewEnumerator2"))
          (:TitleScreen
            ;[0.15 0.15 0.15 0.5] Cast Task
            (bind _asbp_title_screen (Utilities|Casting|CastToBP_TitleScreen (Variables|TouchPressed|GetHitActor)))
            (Variables|CastActor|SetCredits _asbp_title_screen)
            (Variables|CastActor|SetEnumActor "NewEnumerator3")))
        (else
          (goto _label))))
    (:Is%20Not%20Valid
      (goto _label))))

(fn CameraRotationMove
  (bind _output_get (Variables|RotationCamera|SetCurrentPointerLocation (.x (Variables|TouchPressed|GetCurrentTouchPosition))))
  (if (Variables|TouchPressed|GetIsTouchActive)
    (Utilities|FlowControl|Sequence
      (:then_0
        (if (> (- (Variables|RotationCamera|GetFirstPointerLocation) _output_get) (Variables|RotationCamera|GetMovementTreshold))
          (Default|RotateCameratoRight (Variables|Default|GetPlayerCharacter))
          (Variables|TouchPressed|SetIsTouchActive false)))
      (:then_1
        (if (< (- (Variables|RotationCamera|GetFirstPointerLocation) _output_get) (* -1.0 (Variables|RotationCamera|GetMovementTreshold)))
          (Default|RotateCameratoLeft (Variables|Default|GetPlayerCharacter))
          (Variables|TouchPressed|SetIsTouchActive false))))))

(fn CameraRotationPressed
  (Variables|RotationCamera|SetFirstPointerLocation (.x (Variables|TouchPressed|GetStartTouchPosition)))
  (Variables|TouchPressed|SetIsTouchActive true)
  ;[0.15 0.15 0.15 0.5] Makes sure it's a swipe (cancels itself on drag)
  (Components|Timeline|PlayfromStart (Variables|Default|GetDelaySwipeRotationCamera)))