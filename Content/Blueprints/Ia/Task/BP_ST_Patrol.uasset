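; State Tree task that moves an enemy along its patrol points, with a random chance to check for the player instead.
; On entering the state, a roll against the enemy's CurrentPercentCheckPlayer either continues the patrol or sends a CheckPlayer event and fails the task.
; Patrolling advances a wrapping index, loops a walk animation and uses AIMoveTo toward that point's actor, then stops the animation and succeeds when the move finishes.
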(event EventLatentEnterState
  (params (Transition :type State%20Tree%20Transition%20Result%20Structure%20%28by%20ref%29))
  (bind _enemy (Variables|Default|GetEnemy))
  (if (>= (Math|Random|RandomIntegerinRange 0 100) (Variables|/Game/Blueprints/Ia/BP_NPC_Enemy.BP_NPC_Enemy_C|GetCurrentPercentCheckPlayer (Variables|Default|GetEnemy)))
    (Math|Integer|IncrementInt (Variables|/Game/Blueprints/Ia/BP_NPC_Enemy.BP_NPC_Enemy_C|GetIndexPatrol (Variables|Default|GetEnemy))
      (:%20%20
        (if (< (Variables|/Game/Blueprints/Ia/BP_NPC_Enemy.BP_NPC_Enemy_C|GetIndexPatrol (Variables|Default|GetEnemy)) (Utilities|Array|Length (Variables|/Game/Blueprints/Ia/BP_NPC_Enemy.BP_NPC_Enemy_C|GetPatrolKeyLocations (Variables|Default|GetEnemy))))
          _
          (else
            (Variables|/Game/Blueprints/Ia/BP_NPC_Enemy.BP_NPC_Enemy_C|SetIndexPatrol (Variables|Default|GetEnemy) 0)))
        (Components|Animation|PlayAnimation (Variables|/Script/Engine.Character|GetMesh (Variables|Default|GetEnemy)) (Variables|Default|GetWalkAnim) true)
        (AI|AIMoveTo (AI|GetAIController (Variables|Default|GetEnemy)) "0, 0, 0" (Utilities|Array|Get(acopy) (Variables|/Game/Blueprints/Ia/BP_NPC_Enemy.BP_NPC_Enemy_C|GetPatrolKeyLocations _enemy) (Variables|/Game/Blueprints/Ia/BP_NPC_Enemy.BP_NPC_Enemy_C|GetIndexPatrol _enemy)) -1.0 "Default" "Default" true false
          (:OnMoveFinished
            (Audio|Components|Audio|Stop (Variables|/Script/Engine.Character|GetMesh (Variables|Default|GetEnemy)))
            (StateTree|FinishTask true)))))
    (else
      (Class|StateTreeNodeBlueprintBase|SendEvent (Variables|Default|GetCheckPlayer))
      (StateTree|FinishTask false))))