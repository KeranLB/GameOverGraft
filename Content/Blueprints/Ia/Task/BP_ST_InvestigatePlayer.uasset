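; StateTree task where an enemy investigates the player and catches an escape attempt.
; On entering the state, it scans the player character's cuff list and treats an active cuff as escaping, which prints a loss, sends the end event and finishes the task.
; Otherwise it rotates the enemy and plays a left, right or center check animation based on its check point.
; That branch stores the animation length in Delay without finishing the task.
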(event EventLatentEnterState
  (params (Transition :type State%20Tree%20Transition%20Result%20Structure%20%28by%20ref%29))
  (bind _enemy (Variables|Default|GetEnemy))
  (bind _asbp_character (Utilities|Casting|CastToBP_Character (Game|GetPlayerCharacter 0)))
  (for _array_element (Variables|/Game/Blueprints/Player/BP_Character.BP_Character_C|GetCuffList _asbp_character)
    (Variables|/Game/Blueprints/Panels/BP_Cuff.BP_Cuff_C|GetIsActive _array_element
      (:then
        (Variables|Default|SetIsEscaping true))
      (:else)))
  (Variables|Default|GetIsEscaping
    (:then
      ;[0.15 0.15 0.15 0.5] End of the game
      (Development|PrintString "you lose")
      (Class|StateTreeNodeBlueprintBase|SendEvent (Variables|Default|GetEventEnd))
      (StateTree|FinishTask true))
    (:else
      (Utilities|FlowControl|Sequence
        (:then_0
          (switch Utilities|FlowControl|Switch|SwitchonE_ChekPlayerPoints (Variables|/Game/Blueprints/Ia/BP_NPC_Enemy.BP_NPC_Enemy_C|GetPointToCheckPlayer (Variables|Default|GetEnemy))
            (:NewEnumerator0
              (Variables|Default|SetCurrentAnimation (Variables|Default|GetL_Anim))
              (Variables|Default|SetCurrentTargetRotator "0.000000,-90.000000,0.000000"))
            (:NewEnumerator1
              (Variables|Default|SetCurrentAnimation (Variables|Default|GetR_Anim))
              (Variables|Default|SetCurrentTargetRotator "0, 0, 0"))
            (:NewEnumerator2
              (Variables|Default|SetCurrentAnimation (Variables|Default|GetC_Anim))
              (Variables|Default|SetCurrentTargetRotator "0, 0, 0"))))
        (:then_1
          (Transformation|SetWorldRotation (Variables|/Script/Engine.Actor|GetRootComponent _enemy) (Variables|Default|GetCurrentTargetRotator) false false)
          (Components|Animation|PlayAnimation (Variables|/Script/Engine.Character|GetMesh _enemy) (Variables|Default|GetCurrentAnimation) false)
          (bind _output_get (Variables|Output|SetDelay (Animation|GetPlayLength (Variables|Default|GetCurrentAnimation))))
          (Development|PrintString (Utilities|String|ToString(Float) _output_get)))))))