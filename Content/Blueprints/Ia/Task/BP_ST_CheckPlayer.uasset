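; StateTree task that sends an enemy to check on the player at a randomly chosen inspection point.
; On entering the state, it picks left, right or center from a list, stores the choice on the Enemy and resolves the matching location actor.
; It loops a walk animation directly on the mesh during AI MoveTo, then stops it and finishes the task as succeeded when the move finishes.
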(event EventLatentEnterState
  (params (Transition :type State%20Tree%20Transition%20Result%20Structure%20%28by%20ref%29))
  (Utilities|FlowControl|Sequence
    (:then_0
      (bind _output_get (Variables|/Game/Blueprints/Ia/BP_NPC_Enemy.BP_NPC_Enemy_C|SetPointToCheckPlayer (Variables|Default|GetEnemy) (.OutItem (Utilities|Array|Random (Variables|Default|GetlistRandEnum)))))
      (switch Utilities|FlowControl|Switch|SwitchonE_ChekPlayerPoints _output_get
        (:NewEnumerator0
          (Variables|Default|SetActorToGo (Variables|/Game/Blueprints/Ia/BP_NPC_Enemy.BP_NPC_Enemy_C|GetL_InspectPlayerLoc (Variables|Default|GetEnemy))))
        (:NewEnumerator1
          (Variables|Default|SetActorToGo (Variables|/Game/Blueprints/Ia/BP_NPC_Enemy.BP_NPC_Enemy_C|GetRInspectPlayerLoc (Variables|Default|GetEnemy))))
        (:NewEnumerator2
          (Variables|Default|SetActorToGo (Variables|/Game/Blueprints/Ia/BP_NPC_Enemy.BP_NPC_Enemy_C|GetC_InspectPlayerLoc (Variables|Default|GetEnemy))))))
    (:then_1
      (Components|Animation|PlayAnimation (Variables|/Script/Engine.Character|GetMesh (Variables|Default|GetEnemy)) (Variables|Default|GetWalkAnimtion) true)
      (AI|AIMoveTo (AI|GetAIController (Variables|Default|GetEnemy)) "0, 0, 0" (Variables|Default|GetActorToGo) -1.0 "Default" "Default" true true
        (:OnMoveFinished
          (Audio|Components|Audio|Stop (Variables|/Script/Engine.Character|GetMesh (Variables|Default|GetEnemy)))
          (StateTree|FinishTask true))))))