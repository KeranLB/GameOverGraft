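; StateTree task, in a debug folder, that sends an enemy to inspect a location and play an animation there.
; On entering the state, the enemy's AI controller moves it to its RInspectPlayerLoc actor.
; When the move finishes, it plays the task's animation once on the mesh, waits out its length with a Delay, then finishes as succeeded.
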(event EventLatentEnterState
  (params (Transition :type State%20Tree%20Transition%20Result%20Structure%20%28by%20ref%29))
  (bind _anim (Variables|Default|GetAnim))
  (AI|AIMoveTo (AI|GetAIController (Variables|Default|GetEnemy)) "0, 0, 0" (Variables|/Game/Blueprints/Ia/BP_NPC_Enemy.BP_NPC_Enemy_C|GetRInspectPlayerLoc (Variables|Default|GetEnemy)) -1.0 "Default" "Default" true true
    (:OnMoveFinished
      (Components|Animation|PlayAnimation (Variables|/Script/Engine.Character|GetMesh (Variables|Default|GetEnemy)) _anim false)
      (Utilities|FlowControl|Delay (Animation|GetPlayLength _anim))
      (StateTree|FinishTask true))))