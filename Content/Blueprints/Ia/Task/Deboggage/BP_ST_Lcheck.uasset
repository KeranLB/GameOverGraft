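; StateTree task that sends an enemy to its LInspectPlayerLoc actor to play an inspection check.
; On entering the state, it runs AI MoveTo through the enemy's controller toward that goal.
; When the move finishes, it snaps the root component to a fixed world rotation and plays a non-looping animation on the mesh.
; It finishes the task as succeeded after a fixed delay, independent of the animation's length.
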(event EventLatentEnterState
  (params (Transition :type State%20Tree%20Transition%20Result%20Structure%20%28by%20ref%29))
  (AI|AIMoveTo (AI|GetAIController (Variables|Default|GetEnemy)) "0, 0, 0" (Variables|/Game/Blueprints/Ia/BP_NPC_Enemy.BP_NPC_Enemy_C|GetL_InspectPlayerLoc (Variables|Default|GetEnemy)) -1.0 "Default" "Default" true true
    (:OnMoveFinished
      (Transformation|SetWorldRotation (Variables|/Script/Engine.Actor|GetRootComponent (Variables|Default|GetEnemy)) "0.000000,-50.000000,0.000000" false false)
      (Components|Animation|PlayAnimation (Variables|/Script/Engine.Character|GetMesh (Variables|Default|GetEnemy)) (Variables|Default|GetAnim) false)
      (Utilities|FlowControl|Delay 1e+01)
      (StateTree|FinishTask true))))