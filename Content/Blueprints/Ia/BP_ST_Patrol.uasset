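; State Tree task that picks and starts an enemy's next patrol move when its state is entered.
; A random roll against PercentToCheckPlayer sends the enemy to its InspectionPlayerLocation actor instead of continuing the route.
; Otherwise it advances IndexPatrol, wrapping to zero, and moves to that entry in the enemy's PatrolKeyLocations.
; Both branches finish successfully right after issuing SimpleMoveToActor, without waiting for arrival.
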(event EventLatentEnterState
  (params (Transition :type State%20Tree%20Transition%20Result%20Structure%20%28by%20ref%29))
  (bind _enemy (Variables|Default|GetEnemy))
  (bind _enemy_2 (Variables|Default|GetEnemy))
  (if (<= (Math|Random|RandomIntegerinRange 0 100) (Variables|Default|GetPercentToCheckPlayer))
    (AI|Navigation|SimpleMovetoActor (AI|GetAIController _enemy) (Variables|/Game/Blueprints/Ia/BP_NPC_Enemy.BP_NPC_Enemy_C|GetInspectionPlayerLocation _enemy))
    (StateTree|FinishTask true)
    (else
      (Math|Integer|IncrementInt (Variables|/Game/Blueprints/Ia/BP_NPC_Enemy.BP_NPC_Enemy_C|GetIndexPatrol (Variables|Default|GetEnemy))
        (:%20%20
          (if (< (Variables|/Game/Blueprints/Ia/BP_NPC_Enemy.BP_NPC_Enemy_C|GetIndexPatrol (Variables|Default|GetEnemy)) (Utilities|Array|Length (Variables|/Game/Blueprints/Ia/BP_NPC_Enemy.BP_NPC_Enemy_C|GetPatrolKeyLocations (Variables|Default|GetEnemy))))
            _
            (else
              (Variables|/Game/Blueprints/Ia/BP_NPC_Enemy.BP_NPC_Enemy_C|SetIndexPatrol (Variables|Default|GetEnemy) 0)))
          (AI|Navigation|SimpleMovetoActor (AI|GetAIController (Variables|Default|GetEnemy)) (Utilities|Array|Get(acopy) (Variables|/Game/Blueprints/Ia/BP_NPC_Enemy.BP_NPC_Enemy_C|GetPatrolKeyLocations _enemy_2) (Variables|/Game/Blueprints/Ia/BP_NPC_Enemy.BP_NPC_Enemy_C|GetIndexPatrol _enemy_2)))
          (StateTree|FinishTask true))))))