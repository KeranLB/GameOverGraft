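; Enemy NPC that hunts the player, driven by a StateTree with per-state tuning for player checking, inspection time and walk speed.
; On BeginPlay it caches the player character and applies the first state's values from its arrays.
; Every tick it sends its distance to the player's UpdateBpm, apparently a proximity-based heart rate.
; EndGame and FailedTask forward events to the StateTree.
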(event EventBeginPlay
  (bind _asbp_character_k (Utilities|Casting|CastToBP_Character_K (Game|Player|GetPlayerPawn 0)))
  (Variables|Components|SetPlayerCharacter _asbp_character_k)
  (CallFunction|ChangeState))

(event EventTick
  (params (DeltaSeconds :type Float%20%28single-precision%29))
  (bind _distance (CallFunction|GetDistanceEnemy))
  (Default|UpdateBpm (Variables|Components|GetPlayerCharacter) _distance))

(fn ConstructionScript)

(fn GetDistanceEnemy
  (return (Transformation|GetDistanceTo (Variables|Components|GetPlayerCharacter) self)))

(fn EndGame
  (Gameplay|StateTree|SendStateTreeEvent (Variables|Default|GetStateTree) (Variables|Default|GetEndTime) :!class /Script/GameplayStateTreeModule.StateTreeComponent))

(fn FailedTask
  (Gameplay|StateTree|SendStateTreeEvent (Variables|Default|GetStateTree) (Variables|Default|GetTaskError) :!class /Script/GameplayStateTreeModule.StateTreeComponent))

(fn ChangeState
  (params (State :type Integer))
  (Variables|AtomicParameters|SetCurrentPercentCheckPlayer (Utilities|Array|Get(acopy) (Variables|AtomicParameters|GetPercentCheckPlayer) State))
  (Variables|AtomicParameters|SetCurrentInspectionDuration (Utilities|Array|Get(acopy) (Variables|AtomicParameters|GetInspectionDuration) State))
  (bind _output_get (Variables|AtomicParameters|SetCurrentEnemySpeed (Utilities|Array|Get(acopy) (Variables|AtomicParameters|GetEnnemySpeed) State)))
  (Variables|/Script/Engine.CharacterMovementComponent|SetMaxWalkSpeed (Variables|Character|GetCharacterMovement) _output_get))