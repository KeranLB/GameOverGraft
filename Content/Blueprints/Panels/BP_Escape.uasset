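; BP_Escape is a panel Blueprint that turns a Screw component to follow touch drags while IsActive is set.
; EscapePressed records the touch start, and EscapeRotationFollow moves the Rotator component in world X and Z by the scaled drag delta, then resets the start point.
; Screw is re-aimed at Rotator with a look-at rotation, so the moved component serves as an aim target.
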(event EventBeginPlay)

(event Collision|EventActorBeginOverlap
  (params (OtherActor :type Actor%20Object%20Reference)))

(fn ConstructionScript)

(fn EscapePressed
  (params (StartPosition :type Vector%202D%20Structure))
  (if (Variables|Default|GetIsActive)
    (Variables|Default|SetStartTouchPos StartPosition)))

(fn EscapeRotationFollow
  (params (Touch%20Pos :type Vector%202D%20Structure))
  (bind _rotatormovementspeed (Variables|Default|GetRotatorMovementSpeed))
  (bind _rotator (Variables|Default|GetRotator))
  (bind _returnvalue (Transformation|GetWorldLocation _rotator))
  (if (Variables|Default|GetIsActive)
    (Variables|Default|SetCurrentTouchPos Touch%20Pos)
    (Transformation|SetWorldLocation (Variables|Default|GetRotator) (Math|Vector|MakeVector (+ (.x _returnvalue) (* (- (.x (Variables|Default|GetCurrentTouchPos)) (.x (Variables|Default|GetStartTouchPos))) _rotatormovementspeed)) (.y _returnvalue) (+ (.z _returnvalue) (* (- (.y (Variables|Default|GetStartTouchPos)) (.y (Variables|Default|GetCurrentTouchPos))) _rotatormovementspeed))) false false)
    (Variables|Default|SetStartTouchPos (Variables|Default|GetCurrentTouchPos))
    ;[0.15 0.15 0.15 0.5] Makes Screw look at Rotator
    (Transformation|SetWorldRotation (Variables|Default|GetScrew) (Math|Rotator|FindLookatRotation (Transformation|GetWorldLocation (Variables|Default|GetScrew)) (Transformation|GetWorldLocation (Variables|Default|GetRotator))) false false)))