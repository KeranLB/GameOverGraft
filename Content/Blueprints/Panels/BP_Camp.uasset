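; BP_Camp represents a camp with a name and a state of Safe, Attacked or Destroyed.
; On BeginPlay it assigns the camp mesh to its static mesh component.
; ChangeState stores the new state and swaps the mesh's first material to match it.
; GetCampInfos returns the camp's name and current state.
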(event EventBeginPlay
  (Components|StaticMesh|SetStaticMesh (Variables|Default|GetCamp) (Variables|Default|GetCampMesh)))

(fn ConstructionScript)

(fn ChangeState
  (params (CampSate :type E_BasesStatuses%20Enum :default "NewEnumerator0"))
  (bind _output_get (Variables|Default|SetState CampSate))
  (switch Utilities|FlowControl|Switch|SwitchonE_BasesStatuses _output_get
    (:NewEnumerator0
      (Rendering|Material|SetMaterial (Variables|Default|GetCamp) 0 (Variables|Default|GetM_Safe)))
    (:NewEnumerator1
      (Rendering|Material|SetMaterial (Variables|Default|GetCamp) 0 (Variables|Default|GetM_Attacked)))
    (:NewEnumerator2
      (Rendering|Material|SetMaterial (Variables|Default|GetCamp) 0 (Variables|Default|GetM_Destroy)))))

(fn GetCampInfos
  (return (Variables|Default|GetName) (Variables|Default|GetState)))