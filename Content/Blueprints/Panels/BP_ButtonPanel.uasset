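; Touch-operated button panel puzzle where the player matches random codes shown on a screen widget using a lever, a slider and a symbol-cycling button.
; Component tags route presses; timelines animate lever and buttons, and the dragged slider snaps to the nearest of five computed positions on release.
; Validation compares the inputs to the target, generating the next code or, after the last, clearing the screen and notifying the owning task.
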(event EventBeginPlay
  ;[0.15 0.15 0.15 0.5] Set Widget ScreenInfos
  (bind _returnvalue (UserInterface|CreateWidget "/Game/UI/ButtonPanel/WBP_ScreenCodeSymbol.WBP_ScreenCodeSymbol_C"))
  (bind _output_get (Variables|CodeTarget|SetScreenCodeTarget _returnvalue))
  (UserInterface|SetWidget (Variables|CodeManager|GetScreenInfos) _output_get)
  ;[0.15 0.15 0.15 0.5] Set Screen Infos
  (CodeManager|ResetScreenInfos)
  (Slider|SetSliderPositions)
  ;[0.15 0.15 0.15 0.5] Set LeverSwitchSpeed to timeline
  (Components|Timeline|SetPlayRate (Variables|Default|GetLeverSwitchAnim) (/ 1.0 (Variables|AtomicParameters|GetLeverSwitchSpeed)))
  ;[0.15 0.15 0.15 0.5] Set LeverSwitchSpeed to timeline
  (Components|Timeline|SetPlayRate (Variables|Default|GetButtonClickedAnim) (/ 1.0 (Variables|AtomicParameters|GetButtonClickedAnimSpeed))))

(fn ConstructionScript)

(fn ButtonPanelPressed
  (params (StartPoosition :type Vector%202D%20Structure) (ComponentHit :type Primitive%20Component%20Object%20Reference))
  (Variables|Touch|SetTouchStartPosition StartPoosition)
  (switch name (Utilities|Array|Get(acopy) (Variables|/Script/Engine.ActorComponent|GetComponentTags ComponentHit))
    (:Slider
      (Variables|Slider|SetSliderMove true)
      (Variables|Slider|SetSliderPositionX (.x (Variables|/Script/Engine.SceneComponent|GetRelativeLocation (Variables|Slider|GetSM_Slider)))))
    (:ValidationButton
      (ValidationButton|ValidationButtonPressed))
    (:SymbolButton
      (ButtonSymbol|ButtonSymbolPressed))
    (:Lever
      (Lever|LeverSwitch))))

(fn LeverSwitch
  (Variables|Lever|GetCanSwitch
    (:then
      ;[0.15 0.15 0.15 0.5] Switch SliderState
      (Variables|CodeEntry|GetLeverEntry
        (:then
          (Variables|CodeEntry|SetLeverEntry false)
          (Development|PrintString "play animation Switch OFF")
          ;[0.15 0.15 0.15 0.5] Play Animation Lever
          (Variables|Lever|SetCanSwitch false)
          (Components|Timeline|PlayfromStart (Variables|Default|GetLeverSwitchAnim)))
        (:else
          (Variables|CodeEntry|SetLeverEntry true)
          (Development|PrintString "play animation Switch ON")
          (Variables|Lever|SetCanSwitch false)
          (Components|Timeline|ReversefromEnd (Variables|Default|GetLeverSwitchAnim)))))
    (:else)))

(fn ButtonSymbolPressed
  (Variables|Buttons|GetCanClick
    (:then
      (Utilities|FlowControl|Sequence
        (:then_0
          ;[0.15 0.15 0.15 0.5] Play animation
          (Variables|Buttons|SetCanClick false)
          (Variables|Buttons|SetBoutonClicked "NewEnumerator0")
          (Variables|Buttons|SetButtonsPositionYStart (.y (Variables|/Script/Engine.SceneComponent|GetRelativeLocation (Variables|ButtonSymbol|GetSM_ButtonPanel_SymbolButton))))
          (Components|Timeline|PlayfromStart (Variables|Default|GetButtonClickedAnim)))
        (:then_1
          ;[0.15 0.15 0.15 0.5] Increment ButtonSymbolEntry
          (Math|Integer|IncrementInt (Variables|CodeEntry|GetButtonSymbolEntry)
            (:%20%20
              (if (not (<= (Variables|CodeEntry|GetButtonSymbolEntry) 4))
                (Variables|CodeEntry|SetButtonSymbolEntry 0)))))
        (:then_2
          ;[0.15 0.15 0.15 0.5] FeedBack New Value
          (Development|PrintString (Utilities|String|ToString(Integer) (Variables|CodeEntry|GetButtonSymbolEntry))))))
    (:else)))

(fn GenerateCodeTarget
  (params (NbCodeToGenerate :type Integer) (Task :type BP%20Task%20Object%20Reference))
  (Variables|Default|SetNbSymbolToGenerate NbCodeToGenerate)
  (Variables|Default|SetBP_Task Task)
  (Variables|CodeTarget|SetLeverTarget (Math|Random|RandomBool))
  (Variables|CodeTarget|GetLeverTarget
    (:then
      (Variables|CodeTarget|SetLeverIntTarget 1))
    (:else
      (Variables|CodeTarget|SetLeverIntTarget 0)))
  (Variables|CodeTarget|SetSliderTarget (Math|Random|RandomIntegerinRange 0 4))
  (Variables|CodeTarget|SetButtonSymbolTarget (Math|Random|RandomIntegerinRange 0 4))
  (CodeManager|GenerateCodeImage))

(fn GenerateCodeImage
  ;[0.15 0.15 0.15 0.5] Set ButtonSymbol Image
  (Appearance|SetBrushfromTexture (Variables|/Game/UI/ButtonPanel/WBP_ScreenCodeSymbol.WBP_ScreenCodeSymbol_C|GetButtonSymbol (Variables|CodeTarget|GetScreenCodeTarget)) (Utilities|Array|Get(acopy) (Variables|CodeImages|GetButtonSymbolImage) (Variables|CodeTarget|GetButtonSymbolTarget)) false)
  ;[0.15 0.15 0.15 0.5] Set Lever Image
  (Appearance|SetBrushfromTexture (Variables|/Game/UI/ButtonPanel/WBP_ScreenCodeSymbol.WBP_ScreenCodeSymbol_C|GetLeverSymbol (Variables|CodeTarget|GetScreenCodeTarget)) (Utilities|Array|Get(acopy) (Variables|CodeImages|GetLeverImage) (Variables|CodeTarget|GetLeverIntTarget)) false)
  ;[0.15 0.15 0.15 0.5] Set Slider Image
  (Appearance|SetBrushfromTexture (Variables|/Game/UI/ButtonPanel/WBP_ScreenCodeSymbol.WBP_ScreenCodeSymbol_C|GetSliderSymbol (Variables|CodeTarget|GetScreenCodeTarget)) (Utilities|Array|Get(acopy) (Variables|CodeImages|GetSliderImage) (Variables|CodeTarget|GetSliderTarget)) false))

(fn VerifCode
  (return (Math|Boolean|ANDBoolean (== (Variables|CodeEntry|GetLeverEntry) (Variables|CodeTarget|GetLeverTarget)) (== (Variables|CodeEntry|GetSliderEntry) (Variables|CodeTarget|GetSliderTarget)) (== (Variables|CodeEntry|GetButtonSymbolEntry) (Variables|CodeTarget|GetButtonSymbolTarget)))))

(fn ValidationButtonPressed
  (Variables|Buttons|GetCanClick
    (:then
      (Variables|Buttons|SetCanClick false)
      (Variables|Buttons|SetBoutonClicked "NewEnumerator1")
      (Variables|Buttons|SetButtonsPositionYStart (.y (Variables|/Script/Engine.SceneComponent|GetRelativeLocation (Variables|ValidationButton|GetSM_ButtonPanel_ConfirmationButton))))
      (Components|Timeline|PlayfromStart (Variables|Default|GetButtonClickedAnim)))
    (:else)))

(fn SliderFollow
  (params (TouchActualPosition :type Vector%202D%20Structure))
  (bind _sm_slider (Variables|Slider|GetSM_Slider))
  (bind _relativelocation (Variables|/Script/Engine.SceneComponent|GetRelativeLocation _sm_slider))
  (Variables|Slider|GetSliderMove
    (:then
      (Variables|Touch|SetTouchActualPosition TouchActualPosition)
      (bind _output_get (Variables|Slider|SetSliderPositionX (+ (* (- (.x (Variables|Touch|GetTouchActualPosition)) (.x (Variables|Touch|GetTouchStartPosition))) (Variables|AtomicParameters|GetSliderMovementSpeed)) (Variables|Slider|GetSliderPositionX))))
      (Transformation|SetRelativeLocation (Variables|Slider|GetSM_Slider) (Math|Vector|MakeVector (Math|Float|Clamp(Float) _output_get (Variables|Slider|GetSliderPositionXMin) (Variables|Slider|GetSliderPositionXMax)) (.y _relativelocation) (.z _relativelocation)) false false)
      (Variables|Touch|SetTouchStartPosition (Variables|Touch|GetTouchActualPosition)))
    (:else)))

(fn ResetScreenInfos
  (Appearance|SetBrushfromTexture (Variables|/Game/UI/ButtonPanel/WBP_ScreenCodeSymbol.WBP_ScreenCodeSymbol_C|GetButtonSymbol (Variables|CodeTarget|GetScreenCodeTarget)) "/Game/Textures/ButtonsPanelScreen/T_ButtonSymbol_0.T_ButtonSymbol_0" false)
  (Appearance|SetBrushfromTexture (Variables|/Game/UI/ButtonPanel/WBP_ScreenCodeSymbol.WBP_ScreenCodeSymbol_C|GetSliderSymbol (Variables|CodeTarget|GetScreenCodeTarget)) "/Game/Textures/ButtonsPanelScreen/T_ButtonSymbol_0.T_ButtonSymbol_0" false)
  (Appearance|SetBrushfromTexture (Variables|/Game/UI/ButtonPanel/WBP_ScreenCodeSymbol.WBP_ScreenCodeSymbol_C|GetLeverSymbol (Variables|CodeTarget|GetScreenCodeTarget)) "/Game/Textures/ButtonsPanelScreen/T_ButtonSymbol_0.T_ButtonSymbol_0" false))

(fn SliderReleased
  (bind _sm_slider (Variables|Slider|GetSM_Slider))
  (bind _relativelocation (Variables|/Script/Engine.SceneComponent|GetRelativeLocation _sm_slider))
  (Utilities|FlowControl|Sequence
    (:then_0
      ;[0.15 0.15 0.15 0.5] Get SM_Slider Position X
      (Variables|Slider|SetKeyValue (.x (Variables|/Script/Engine.SceneComponent|GetRelativeLocation (Variables|Slider|GetSM_Slider)))))
    (:then_1
      ;[0.15 0.15 0.15 0.5] Look for Key position framing actual position of SM_Slider position X
      (bind _index (Utilities|FlowControl|ForLoopwithBreak 0 3 :!label _label)
        (:LoopBody
          (Variables|CodeEntry|SetSliderEntry _index)
          (if (and (<= (Utilities|Array|Get(acopy) (Variables|Slider|GetKeyPosition) _index) (Variables|Slider|GetKeyValue)) (<= (Variables|Slider|GetKeyValue) (Utilities|Array|Get(acopy) (Variables|Slider|GetKeyPosition) (+ _index 1))))
            (goto _label Break)))))
    (:then_2
      ;[0.15 0.15 0.15 0.5] find the closer Key Position Betwin the two frame
      (if (not (<= (Variables|Slider|GetKeyValue) (+ (/ (- (Utilities|Array|Get(acopy) (Variables|Slider|GetKeyPosition) (+ (Variables|CodeEntry|GetSliderEntry) 1)) (Utilities|Array|Get(acopy) (Variables|Slider|GetKeyPosition) (Variables|CodeEntry|GetSliderEntry))) 2.0) (Utilities|Array|Get(acopy) (Variables|Slider|GetKeyPosition) (Variables|CodeEntry|GetSliderEntry)))))
        (Math|Integer|IncrementInt (Variables|CodeEntry|GetSliderEntry))))
    (:then_3
      ;[0.15 0.15 0.15 0.5] Set SM_Slider to the right X position
      (Transformation|SetRelativeLocation (Variables|Slider|GetSM_Slider) (Math|Vector|MakeVector (Utilities|Array|Get(acopy) (Variables|Slider|GetKeyPosition) (Variables|CodeEntry|GetSliderEntry)) (.y _relativelocation) (.z _relativelocation)) false false)
      (Variables|Slider|SetSliderMove false))))

(fn SetSliderPositions
  (Utilities|FlowControl|Sequence
    (:then_0
      ;[0.15 0.15 0.15 0.5] Set Key position Interval
      (Variables|Slider|SetKeyPositionInterval (/ (- (Variables|Slider|GetSliderPositionXMax) (Variables|Slider|GetSliderPositionXMin)) 4.0)))
    (:then_1
      ;[0.15 0.15 0.15 0.5] Set Key's positions
      (Variables|Slider|SetKeyValue (Variables|Slider|GetSliderPositionXMin))
      (for _index (range 0 4)
        (Utilities|Array|SetArrayElem (Variables|Slider|GetKeyPosition) _index (Variables|Slider|GetKeyValue))
        (Variables|Slider|SetKeyValue (+ (Variables|Slider|GetKeyValue) (Variables|Slider|GetKeyPositionInterval)))))))

(fn ButtonPanelReleased
  (Variables|Slider|GetSliderMove
    (:then
      (Slider|SliderReleased))
    (:else)))

(fn SymbolButtonAnimation
  (params (Alpha :type Float%20%28double-precision%29))
  (bind _sm_buttonpanel_symbolbutton (Variables|ButtonSymbol|GetSM_ButtonPanel_SymbolButton))
  (bind _buttonspositionystart (Variables|Buttons|GetButtonsPositionYStart))
  (bind _relativelocation (Variables|/Script/Engine.SceneComponent|GetRelativeLocation _sm_buttonpanel_symbolbutton))
  ;[0.15 0.15 0.15 0.5] Update ButtonClickedAnim
  (Transformation|SetRelativeLocation (Variables|ButtonSymbol|GetSM_ButtonPanel_SymbolButton) (Math|Vector|MakeVector (.x _relativelocation) (Math|Float|Lerp _buttonspositionystart (- _buttonspositionystart (Variables|Buttons|GetButtonClickedDeepTarget)) Alpha) (.z _relativelocation)) false false))

(fn ValidationButtonAnimation
  (params (Alpha :type Float%20%28double-precision%29))
  (bind _sm_buttonpanel_confirmationbutton (Variables|ValidationButton|GetSM_ButtonPanel_ConfirmationButton))
  (bind _buttonspositionystart (Variables|Buttons|GetButtonsPositionYStart))
  (bind _relativelocation (Variables|/Script/Engine.SceneComponent|GetRelativeLocation _sm_buttonpanel_confirmationbutton))
  ;[0.15 0.15 0.15 0.5] Update ButtonClickedAnim
  (Transformation|SetRelativeLocation (Variables|ValidationButton|GetSM_ButtonPanel_ConfirmationButton) (Math|Vector|MakeVector (.x _relativelocation) (Math|Float|Lerp _buttonspositionystart (- _buttonspositionystart (Variables|Buttons|GetButtonClickedDeepTarget)) Alpha) (.z _relativelocation)) false false))

(fn GiveInfostoTask
  (Default|CheckStep (Variables|Default|GetBP_Task)))