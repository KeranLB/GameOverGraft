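; BP_Screw is a touch-driven screw actor that the player unscrews by circling a finger around it.
; While active and touched, it compares touch directions around the screw's projected screen position using atan2 of cross and dot products.
; Only positive deltas, scaled by sensitivity, rotate the actor's pitch and add to its accumulated angle.
; At the maximum angle it locks as unscrewed and sets its indexed win condition on the parent cuff.
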(event EventBeginPlay)

(event Collision|EventActorBeginOverlap
  (params (OtherActor :type Actor%20Object%20Reference)))

(fn ConstructionScript)

(fn ScrewPressed
  (params (StartPosition :type Vector%202D%20Structure))
  (if (Variables|Default|GetIsActive)
    (Variables|Input|SetStartTouchPos StartPosition)
    ;[0.15 0.15 0.15 0.5] 3D world to 2D Screen location
    (Variables|AngleComputing|SetScrew%20Screen%20Location (.ScreenLocation (Class|PlayerController|ProjectWorldLocationtoScreen (Game|GetPlayerController 0) (Transformation|GetWorldLocation (Variables|Default|GetScrew)) false)))
    (Variables|AngleComputing|SetLastDirection (- (Variables|AngleComputing|GetScrew%20Screen%20Location) (Variables|Input|GetStartTouchPos)))
    (Variables|Default|SetIsTouching true)))

(fn ScrewRotationFollow
  (params (Touch%20Pos :type Vector%202D%20Structure))
  (if (Variables|Default|GetIsActive)
    (if (not (Variables|Default|GetIsUnscrewed))
      (if (Variables|Default|GetIsTouching)
        (bind _output_get (Variables|Input|SetCurrentTouchPos Touch%20Pos))
        (Variables|AngleComputing|SetCurrentDirection (Math|Vector2D|Normalize2D (- _output_get (Variables|AngleComputing|GetScrew%20Screen%20Location))))
        ;[0.15 0.15 0.15 0.5] Rotation Delta
        (bind _output_get_2 (Variables|AngleComputing|SetDelta%20Rotation%20Y%20%28Pitch%29 (Class|KismetMathLibrary|DegAtan2 (- (* (.x (Variables|AngleComputing|GetLastDirection)) (.y (Variables|AngleComputing|GetCurrentDirection))) (* (.y (Variables|AngleComputing|GetLastDirection)) (.x (Variables|AngleComputing|GetCurrentDirection)))) (+ (* (.x (Variables|AngleComputing|GetLastDirection)) (.x (Variables|AngleComputing|GetCurrentDirection))) (* (.y (Variables|AngleComputing|GetLastDirection)) (.y (Variables|AngleComputing|GetCurrentDirection)))))))
        ;[0.15 0.15 0.15 0.5] Counterclockwise?
        (if (> _output_get_2 0.0)
          ;[0.15 0.15 0.15 0.5] How much the screw will be rotated
          (Variables|AngleComputing|SetRotationAmount (* (Variables|AngleComputing|GetDelta%20Rotation%20Y%20%28Pitch%29) (Variables|AtomicParameters|GetRotationSensivity)))
          ;[0.15 0.15 0.15 0.5] How much the screw has rotated so far
          (Variables|AngleComputing|SetScrewCurrentAngle (+ (Variables|AngleComputing|GetScrewCurrentAngle) (Variables|AngleComputing|GetRotationAmount)))
          ;[0.15 0.15 0.15 0.5] Actual Rotation
          (Transformation|AddActorLocalRotation (Math|Rotator|MakeRotator 0.0 (Variables|AngleComputing|GetRotationAmount) 0.0) false false)
          ;[0.15 0.15 0.15 0.5] Updates Pointer Position
          (Variables|Input|SetStartTouchPos (Variables|Input|GetCurrentTouchPos))
          (Variables|AngleComputing|SetLastDirection (- (Variables|AngleComputing|GetScrew%20Screen%20Location) (Variables|Input|GetStartTouchPos)))
          ;[0.15 0.15 0.15 0.5] Is the actor's rotation completed
          (if (>= (Variables|AngleComputing|GetScrewCurrentAngle) (Variables|AtomicParameters|GetScrewMaxAngle))
            ;[0.15 0.15 0.15 0.5] Update win condition
            (bind _output_get_3 (Variables|Default|SetIsUnscrewed true))
            (Default|SetWinCond (Variables|Default|GetParent%20Cuff) (Variables|Default|GetScrew%20Index%20in%20Cuff) _output_get_3)))))))

(fn ScrewReleased
  (Variables|Default|SetIsTouching false))

(fn ActivateSelf
  (params (SetBool :type Boolean))
  (Variables|Default|SetIsActive SetBool))

(fn SetParentCuff
  (params (ParentCuff :type BP%20Cuff%20Object%20Reference) (ScrewIndex :type Integer))
  (Variables|Default|SetParent%20Cuff ParentCuff)
  (Variables|Default|SetScrew%20Index%20in%20Cuff ScrewIndex))