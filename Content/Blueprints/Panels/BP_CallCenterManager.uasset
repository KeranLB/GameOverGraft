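; Call center manager that spawns incoming calls at random intervals across a set of caller slots.
; BeginPlay indexes each slot and starts the DelayNewCall timeline, used as a timer by randomizing its play rate between the min and max call delays.
; When it finishes, FindFreeSlot randomly picks one of five untaken slots, triggers its CallEntrance and counts the task.
; Freeslot releases a slot and decrements the count.
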(event EventBeginPlay
  (bind _delaynewcall (Variables|Default|GetDelayNewCall))
  (Components|Timeline|SetPlayRate _delaynewcall 1.0)
  (Components|Timeline|PlayfromStart _delaynewcall)
  ;[0.15 0.15 0.15 0.5] Gives their index to each call center
  (for (_array_element _array_index) (Variables|CallerSlots|GetCallerSlots)
    (Variables|/Game/Blueprints/Panels/BP_CallCenter.BP_CallCenter_C|SetCallCenterIndex _array_element _array_index)))

(fn ConstructionScript)

(fn FindFreeSlot
  (bind _output_get (LocalVariables|SetCurrentIndex (Math|Random|RandomIntegerinRange 0 4) :!label _label))
  (if (Utilities|Array|Get(acopy) (Variables|CallerSlots|GetIsSlotTaken) _output_get)
    ;[0.15 0.15 0.15 0.5] Has empty slot ?
    (if (!= (Utilities|Array|FindItem (Variables|CallerSlots|GetIsSlotTaken) false) -1)
      (goto _label)
      (else
        (return -1)))
    (else
      (return (LocalVariables|GetCurrentIndex)))))

(fn Freeslot
  (params (Index :type Integer))
  (Math|Integer|DecrementInt (Variables|Default|GetNbOfTasks)
    (:%20%20
      (Utilities|Array|SetArrayElem (Variables|CallerSlots|GetIsSlotTaken) Index false))))