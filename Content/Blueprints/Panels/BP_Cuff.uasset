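; BP_Cuff is a cuff puzzle piece with two child BP_Screw actors, which it positions and registers with itself at BeginPlay.
; Pressing it toggles the screws, the visibility of the cuff's child components and the M character's in-use flag, while release is forwarded to both screws.
; SetWinCond records per-screw results, sets IsFree and calls BP_Character_M's win check.
; BP_Character_K is cached, but its win check is unreachable.
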(event EventBeginPlay
  (bind _returnvalue (Game|Player|GetPlayerPawn 0))
  (bind _screwspositions (Variables|Default|GetScrewsPositions))
  ;[0.15 0.15 0.15 0.5] Places the screws in the right spot
  (Transformation|SetRelativeLocation (Variables|Default|GetScrew_1) (Utilities|Array|Get(acopy) _screwspositions) false false)
  (Transformation|SetRelativeLocation (Variables|Default|GetScrew_2) (Utilities|Array|Get(acopy) _screwspositions 1) false false)
  ;[0.15 0.15 0.15 0.5] player K
  (bind _asbp_character_k (Utilities|Casting|CastToBP_Character_K _returnvalue)
    (:then
      (Variables|Default|SetPlayer%20Character _asbp_character_k)
      (bind _asbp_screw (Utilities|Casting|CastToBP_Screw (Variables|/Script/Engine.ChildActorComponent|GetChildActor (Variables|Default|GetScrew_1))))
      (bind _output_get (Variables|Default|SetBP%20Screw%201 _asbp_screw))
      (Default|SetParentCuff _output_get self)
      (bind _asbp_screw_2 (Utilities|Casting|CastToBP_Screw (Variables|/Script/Engine.ChildActorComponent|GetChildActor (Variables|Default|GetScrew_2))))
      (bind _output_get_2 (Variables|Default|SetBP%20Screw%202 _asbp_screw_2))
      (Default|SetParentCuff _output_get_2 self 1))
    (:CastFailed
      ;[0.15 0.15 0.15 0.5] player M
      (bind _asbp_character_m (Utilities|Casting|CastToBP_Character_M _returnvalue))
      (Variables|Default|SetAs%20BP%20Character%20M _asbp_character_m)
      (bind _asbp_screw_3 (Utilities|Casting|CastToBP_Screw (Variables|/Script/Engine.ChildActorComponent|GetChildActor (Variables|Default|GetScrew_1))))
      (bind _output_get_3 (Variables|Default|SetBP%20Screw%201 _asbp_screw_3))
      (Default|SetParentCuff _output_get_3 self)
      (bind _asbp_screw_4 (Utilities|Casting|CastToBP_Screw (Variables|/Script/Engine.ChildActorComponent|GetChildActor (Variables|Default|GetScrew_2))))
      (bind _output_get_4 (Variables|Default|SetBP%20Screw%202 _asbp_screw_4))
      (Default|SetParentCuff _output_get_4 self 1))))

(fn ConstructionScript)

(fn CuffPressed
  (if (Variables|Default|GetIsActive)
    (CallFunction|ToggleScrews false)
    (else
      (CallFunction|ToggleScrews true)))
  (Development|PrintString "Hello"))

(fn ToggleScrews
  (params (Activate? :type Boolean))
  (Default|ActivateSelf (Variables|Default|GetBP%20Screw%201) Activate?)
  (Default|ActivateSelf (Variables|Default|GetBP%20Screw%202) Activate?)
  (for _array_element (Components|GetChildrenComponents (Variables|Default|GetCuff) false)
    (Rendering|SetVisibility _array_element Activate? false)
    (Variables|/Game/Blueprints/Player/BP_Character_M.BP_Character_M_C|SetAreCuffsInUse (Variables|Default|GetAs%20BP%20Character%20M) Activate?)
    (Variables|Default|SetIsActive Activate?)))

(fn SetWinCond
  (params (Index :type Integer) (True? :type Boolean))
  (Utilities|Array|SetArrayElem (Variables|Default|GetWinConditions) Index True?)
  (bind _array_element (Utilities|Array|ForEachLoopwithBreak (Variables|Default|GetWinConditions) :!label _label)
    (:LoopBody
      (if (not _array_element)
        (goto _label Break)))
    (:Completed
      (Variables|Default|SetIsFree true)
      (Default|CheckWinConditions (Variables|Default|GetAs%20BP%20Character%20M)))))

(fn CuffReleased
  (params (HitComponent :type Primitive%20Component%20Object%20Reference))
  (if (== (Utilities|Array|Get(acopy) (Variables|/Script/Engine.ActorComponent|GetComponentTags HitComponent)) "Screw")
    (Default|ScrewReleased (Variables|Default|GetBP%20Screw%201))
    (Default|ScrewReleased (Variables|Default|GetBP%20Screw%202))))

(fn SetParameters
  (bind _maxangle (Variables|Default|GetMaxAngle))
  (bind _sensivity (Variables|Default|GetSensivity))
  (bind _asbp_screw (Utilities|Casting|CastToBP_Screw (Variables|/Script/Engine.ChildActorComponent|GetChildActor (Variables|Default|GetScrew_1))))
  (Variables|/Game/Blueprints/Panels/BP_Screw.BP_Screw_C|SetScrewMaxAngle _asbp_screw _maxangle)
  (Variables|/Game/Blueprints/Panels/BP_Screw.BP_Screw_C|SetRotationSensivity _asbp_screw _sensivity)
  (bind _asbp_screw_2 (Utilities|Casting|CastToBP_Screw (Variables|/Script/Engine.ChildActorComponent|GetChildActor (Variables|Default|GetScrew_2))))
  (Variables|/Game/Blueprints/Panels/BP_Screw.BP_Screw_C|SetScrewMaxAngle _asbp_screw_2 _maxangle)
  (Variables|/Game/Blueprints/Panels/BP_Screw.BP_Screw_C|SetRotationSensivity _asbp_screw_2 _sensivity))