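; Call center switchboard module with an answer button, a draggable cable and a socket for other modules' cables.
; CallEntrance opens a timed answer window, during which the button spawns a task through TaskManager; the missed-call penalty is only a comment.
; Socket overlaps give the incoming cable's module its callee and snap transform.
; Releasing the cable snaps it, activates the task and sets IsInDialogue if the callee matches TargetCall.
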(event OnComponentBeginOverlap(Emplacement)
  (params (OverlappedComponent :type Primitive%20Component%20Object%20Reference) (OtherActor :type Actor%20Object%20Reference) (OtherComp :type Primitive%20Component%20Object%20Reference) (OtherBodyIndex :type Integer) (bFromSweep :type Boolean) (SweepResult :type Hit%20Result%20Structure%20%28by%20ref%29))
  ;[0.15 0.15 0.15 0.5] President Emplacement
  (bind _asbp_call_center (Utilities|Casting|CastToBP_CallCenter OtherActor))
  (Variables|Emplacement|GetIsTaken
    (:then)
    (:else
      (Variables|Emplacement|SetIsTaken true)
      (Variables|Emplacement|SetPersonReceived (Variables|BP_CallCenter_C|GetCallManagerSlot _asbp_call_center))
      (Variables|BP_CallCenter_C|SetPersonCalled _asbp_call_center (Variables|Emplacement|GetCallManagerSlot))
      (Variables|BP_CallCenter_C|SetReleasedPosition _asbp_call_center (Transformation|GetWorldLocation (Variables|Emplacement|GetEmplacement)))
      (Variables|BP_CallCenter_C|SetReleasedRotation _asbp_call_center "0.000000,180.000000,-90.000000"))))

(event OnComponentEndOverlap(Emplacement)
  (params (OverlappedComponent :type Primitive%20Component%20Object%20Reference) (OtherActor :type Actor%20Object%20Reference) (OtherComp :type Primitive%20Component%20Object%20Reference) (OtherBodyIndex :type Integer))
  ;[0.15 0.15 0.15 0.5] President Emplacement
  (bind _asbp_call_center (Utilities|Casting|CastToBP_CallCenter OtherActor))
  (if (Utilities|Enum|Equal(Enum) (Variables|BP_CallCenter_C|GetCallManagerSlot _asbp_call_center) (Variables|Emplacement|GetPersonReceived))
    (Variables|Emplacement|GetIsTaken
      (:then
        (Variables|Emplacement|SetIsTaken false)
        (Variables|Emplacement|SetPersonReceived "NewEnumerator5")
        (Variables|BP_CallCenter_C|SetPersonCalled _asbp_call_center "NewEnumerator5")
        (Variables|BP_CallCenter_C|SetReleasedPosition _asbp_call_center (Variables|BP_CallCenter_C|GetStartPositionCable _asbp_call_center))
        (Variables|BP_CallCenter_C|SetReleasedRotation _asbp_call_center "0.000000,180.000000,20.000000"))
      (:else))))

(event Custom|CallEntrance
  ;[0.15 0.15 0.15 0.5] Set the module ready for task giving
  ; Delay used to remove this state and punish player
  (Development|PrintString (Utilities|String|EnumtoString (Variables|Emplacement|GetCallManagerSlot)))
  (Variables|Default|SetGetCall true)
  (Utilities|FlowControl|Delay (Variables|Default|GetCallWaitDuration))
  (Variables|Default|GetGetCall
    (:then
      ;;[0.15 0.15 0.15 0.5] New error add to jauge
      (Variables|Default|SetGetCall false))
    (:else)))

(event EventBeginPlay
  (bind _output_get (Variables|Cable|SetStartPositionCable (Transformation|GetWorldLocation (Variables|Default|GetSM_BaseCable))))
  (Variables|Cable|SetReleasedPosition _output_get)
  (Variables|Animation|SetStartPosAnim (.y (Variables|/Script/Engine.SceneComponent|GetRelativeLocation (Variables|Default|GetSM_CallAnswerButton))))
  (Components|Timeline|SetPlayRate (Variables|Default|GetButtonCallAnswerAnim) (/ 1.0 (Variables|Animation|GetAnimationSpeed))))

(fn ConstructionScript)

(fn CallCenterPressed
  (params (StartPosition :type Vector%202D%20Structure) (HitCompo :type Primitive%20Component%20Object%20Reference))
  (Variables|CableFollow|SetStartPosition StartPosition)
  (Variables|Cable|GetIsInDialogue
    (:then)
    (:else
      (switch name (Utilities|Array|Get(acopy) (Variables|/Script/Engine.ActorComponent|GetComponentTags HitCompo))
        (:Cable
          (Variables|CableFollow|SetCanCableFollow true)
          (Transformation|SetRelativeRotation (Variables|Default|GetSM_BaseCable) "0.000000,180.000000,90.000000" false false))
        (:AnswerButton
          (CallManager|AnswerButton))))))

(fn AnswerButton
  (Variables|Animation|GetIsClicking
    (:then)
    (:else
      (Variables|Animation|SetIsClicking true)
      (Components|Timeline|PlayfromStart (Variables|Default|GetButtonCallAnswerAnim))
      (Variables|Default|GetGetCall
        (:then
          (bind _outputtask (Default|SpawnTask (Variables|Manager|GetTaskManager)))
          (Variables|Default|SetOutput%20Task _outputtask)
          (Variables|Default|SetGetCall false))
        (:else)))))

(fn CallCenterReleased
  (Variables|CableFollow|GetCanCableFollow
    (:then
      (Variables|CableFollow|SetCanCableFollow false)
      (Transformation|SetWorldLocationAndRotation (Variables|Default|GetSM_BaseCable) (Variables|Cable|GetReleasedPosition) (Variables|Cable|GetReleasedRotation) false false)
      (bind _isgoodreceiver (CallManager|VerifCall))
      (Variables|Cable|SetIsInDialogue _isgoodreceiver))
    (:else)))

(fn CableFollow
  (params (ActualPosition :type Vector%202D%20Structure))
  (Variables|CableFollow|GetCanCableFollow
    (:then
      (Variables|CableFollow|SetActualPosition ActualPosition)
      (Transformation|AddRelativeLocation (Variables|Default|GetSM_BaseCable) (Math|Vector|MakeVector (.x (* (Math|Vector2D|MakeVector2D (- (.x (Variables|CableFollow|GetActualPosition)) (.x (Variables|CableFollow|GetStartPosition))) (- (.y (Variables|CableFollow|GetStartPosition)) (.y (Variables|CableFollow|GetActualPosition)))) (Variables|CableFollow|GetCableFollowSpeed))) 0.0 (.y (* (Math|Vector2D|MakeVector2D (- (.x (Variables|CableFollow|GetActualPosition)) (.x (Variables|CableFollow|GetStartPosition))) (- (.y (Variables|CableFollow|GetStartPosition)) (.y (Variables|CableFollow|GetActualPosition)))) (Variables|CableFollow|GetCableFollowSpeed)))) false false)
      (Variables|CableFollow|SetStartPosition (Variables|CableFollow|GetActualPosition)))
    (:else)))

(fn VerifCall
  ;[0.15 0.15 0.15 0.5] Will be moved to :  EndDialogue
  (Default|Activate (Variables|Default|GetOutput%20Task))
  (return (and (Utilities|Enum|NotEqual(Enum) (Variables|Components|GetTargetCall) "NewEnumerator5") (Utilities|Enum|Equal(Enum) (Variables|Components|GetPersonCalled) (Variables|Components|GetTargetCall)))))

(fn EndConnection
  (Transformation|SetWorldLocationAndRotation (Variables|Default|GetSM_BaseCable) (Variables|Cable|GetStartPositionCable) "0.000000,180.000000,20.000000" false false))