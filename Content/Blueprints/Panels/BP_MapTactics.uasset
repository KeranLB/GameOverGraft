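; BP_MapTactics is an interactive map panel for selecting camps and setting their Safe, Attacked or Destroyed state.
; A capsule overlap selects the camp and displays its name.
; Presses route by component tag to animated buttons or map dragging, with confirmation sending camp and state to TaskManager.
; Dragging rotates the map, and a timeline-delayed position sample gives release inertia above a threshold.
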(event OnComponentBeginOverlap(Capsule)
  (params (OverlappedComponent :type Primitive%20Component%20Object%20Reference) (OtherActor :type Actor%20Object%20Reference) (OtherComp :type Primitive%20Component%20Object%20Reference) (OtherBodyIndex :type Integer) (bFromSweep :type Boolean) (SweepResult :type Hit%20Result%20Structure%20%28by%20ref%29))
  ;[0.15 0.15 0.15 0.5] Aim Camp Manager
  (bind _asbp_camp (Utilities|Casting|CastToBP_Camp OtherActor))
  (bind _output_get (Variables|Map|SetCampSelected _asbp_camp))
  (bind _name (Default|GetCampInfos _output_get))
  (bind _output_get_2 (Variables|Camp|SetEmptyText (Utilities|Text|ToText(String) (Utilities|String|EnumtoString _name))))
  (Rendering|Components|TextRender|SetText (Variables|Default|GetTextRender) _output_get_2))

(event OnComponentEndOverlap(Capsule)
  (params (OverlappedComponent :type Primitive%20Component%20Object%20Reference) (OtherActor :type Actor%20Object%20Reference) (OtherComp :type Primitive%20Component%20Object%20Reference) (OtherBodyIndex :type Integer))
  ;[0.15 0.15 0.15 0.5] Aim Camp Manager
  (Utilities|Casting|CastToBP_Camp OtherActor)
  (Variables|Map|SetCampSelected 0)
  (bind _output_get (Variables|Camp|SetEmptyText ""))
  (Rendering|Components|TextRender|SetText (Variables|Default|GetTextRender) _output_get))

(event EventBeginPlay
  ;[0.15 0.15 0.15 0.5] Begin Play
  ;;[0.15 0.15 0.15 0.5] Set Delay Delta Position
  (Components|Timeline|SetPlayRate (Variables|Default|GetDelayDeltaPosition) (/ 1.0 (Variables|Touch|GetDurationDelayDeltaLocation)))
  ;;[0.15 0.15 0.15 0.5] Set Map Rotation Inertia
  (Components|Timeline|SetPlayRate (Variables|Default|GetMapRotationInertia) (/ 1.0 (Variables|Inertia|GetInertiaDuration)))
  ;;[0.15 0.15 0.15 0.5] Set Button Animation Speed
  (Components|Timeline|SetPlayRate (Variables|Default|GetButtonClickedAnim) (/ 1.0 (Variables|Animation|GetButtonAnimationSpeed))))

(fn ConstructionScript)

(fn MapRotationFollow
  (params (ActualPosition :type Vector%202D%20Structure))
  (bind _maprotationspeed (Variables|Map|GetMapRotationSpeed))
  (Variables|Touch|SetActualPosition ActualPosition)
  (Variables|Map|GetMapRotation
    (:then
      (Transformation|AddWorldRotation (Variables|Default|GetSM_Map) (Math|Rotator|MakeRotator 0.0 0.0 (* (- (.x (Variables|Touch|GetStartPosition)) (.x (Variables|Touch|GetActualPosition))) _maprotationspeed)) false false)
      (Transformation|AddRelativeRotation (Variables|Default|GetSM_Map) (Math|Rotator|MakeRotator 0.0 0.0 (* _maprotationspeed (- (.y (Variables|Touch|GetStartPosition)) (.y (Variables|Touch|GetActualPosition))))) false false)
      (Variables|Touch|SetStartPosition (Variables|Touch|GetActualPosition)))
    (:else)))

(fn MapTacticPressed
  (params (HitComponent :type Primitive%20Component%20Object%20Reference) (StartPosition :type Vector%202D%20Structure))
  (LocalVariables|SetComponentHit HitComponent)
  (Utilities|FlowControl|Sequence
    (:then_0
      (switch name (Utilities|Array|Get(acopy) (Variables|/Script/Engine.ActorComponent|GetComponentTags (LocalVariables|GetComponentHit)))
        (:SafeButton
          (Variables|Animation|SetEnumButtonClicked "NewEnumerator5"))
        (:AttackedButton
          (Variables|Animation|SetEnumButtonClicked "NewEnumerator6"))
        (:DestroyedButton
          (Variables|Animation|SetEnumButtonClicked "NewEnumerator7"))
        (:ValidationButton
          (Variables|Animation|SetEnumButtonClicked "NewEnumerator2"))
        (:Map
          (Variables|Animation|SetEnumButtonClicked "NewEnumerator4"))))
    (:then_1
      (switch Utilities|FlowControl|Switch|SwitchonE_ButtonClicked (Variables|Animation|GetEnumButtonClicked)
        (:NewEnumerator2
          ;[0.15 0.15 0.15 0.5] Confirmation Button
          (Variables|Animation|GetCanClick
            (:then
              (Variables|Animation|SetCanClick false)
              (Map|ConfirmationButtonPressed)
              (Variables|Animation|SetButtonClicked (LocalVariables|GetComponentHit))
              (Variables|Animation|SetStartPositionAnim (Math|Vector2D|MakeVector2D (.y (Variables|/Script/Engine.SceneComponent|GetRelativeLocation (LocalVariables|GetComponentHit))) (.z (Variables|/Script/Engine.SceneComponent|GetRelativeLocation (LocalVariables|GetComponentHit)))))
              (Components|Timeline|PlayfromStart (Variables|Default|GetButtonClickedAnim)))
            (:else)))
        (:NewEnumerator5
          ;[0.15 0.15 0.15 0.5] SafeButton
          (Variables|Animation|GetCanClick
            (:then
              (Variables|Animation|SetCanClick false)
              (bind _campselected (Variables|Map|GetCampSelected)
                (:then
                  (Default|ChangeState _campselected "NewEnumerator0")
                  (Variables|Animation|SetButtonClicked (LocalVariables|GetComponentHit))
                  (Variables|Animation|SetStartPositionAnim (Math|Vector2D|MakeVector2D (.y (Variables|/Script/Engine.SceneComponent|GetRelativeLocation (LocalVariables|GetComponentHit))) (.z (Variables|/Script/Engine.SceneComponent|GetRelativeLocation (LocalVariables|GetComponentHit)))))
                  (Components|Timeline|PlayfromStart (Variables|Default|GetButtonClickedAnim)))
                (:else)))
            (:else)))
        (:NewEnumerator6
          ;[0.15 0.15 0.15 0.5] AttackButton
          (Variables|Animation|GetCanClick
            (:then
              (Variables|Animation|SetCanClick false)
              (bind _campselected_2 (Variables|Map|GetCampSelected)
                (:then
                  (Default|ChangeState _campselected_2 "NewEnumerator1")
                  (Variables|Animation|SetButtonClicked (LocalVariables|GetComponentHit))
                  (Variables|Animation|SetStartPositionAnim (Math|Vector2D|MakeVector2D (.y (Variables|/Script/Engine.SceneComponent|GetRelativeLocation (LocalVariables|GetComponentHit))) (.z (Variables|/Script/Engine.SceneComponent|GetRelativeLocation (LocalVariables|GetComponentHit)))))
                  (Components|Timeline|PlayfromStart (Variables|Default|GetButtonClickedAnim)))
                (:else)))
            (:else)))
        (:NewEnumerator7
          ;[0.15 0.15 0.15 0.5] DestroyButton
          (Variables|Animation|GetCanClick
            (:then
              (Variables|Animation|SetCanClick false)
              (bind _campselected_3 (Variables|Map|GetCampSelected)
                (:then
                  (Default|ChangeState _campselected_3 "NewEnumerator2")
                  (Variables|Animation|SetButtonClicked (LocalVariables|GetComponentHit))
                  (Variables|Animation|SetStartPositionAnim (Math|Vector2D|MakeVector2D (.y (Variables|/Script/Engine.SceneComponent|GetRelativeLocation (LocalVariables|GetComponentHit))) (.z (Variables|/Script/Engine.SceneComponent|GetRelativeLocation (LocalVariables|GetComponentHit)))))
                  (Components|Timeline|PlayfromStart (Variables|Default|GetButtonClickedAnim)))
                (:else)))
            (:else)))
        (:NewEnumerator4
          ;[0.15 0.15 0.15 0.5] Start Map Rotation
          (bind _output_get (Variables|Touch|SetStartPosition StartPosition))
          (Variables|Inertia|SetInertiaDeltaPosition _output_get)
          (Components|Timeline|PlayfromStart (Variables|Default|GetDelayDeltaPosition))
          (Audio|Components|Audio|Stop (Variables|Default|GetMapRotationInertia))
          (Variables|Map|SetMapRotation true))))))

(fn MapTacticReleased
  (params (ActualTouchPosition :type Vector%202D%20Structure))
  (bind _inertiatreshold (Variables|Inertia|GetInertiaTreshold))
  (Variables|Touch|SetActualPosition ActualTouchPosition)
  (Variables|Map|GetMapRotation
    (:then
      (Variables|Inertia|SetInertiaDirection (/ (- (Variables|Inertia|GetInertiaDeltaPosition) (Variables|Touch|GetActualPosition)) (Variables|Inertia|GetInertiaDiminutionSpeed)))
      (if (Math|Boolean|ORBoolean (>= (.x (Variables|Inertia|GetInertiaDirection)) (.x _inertiatreshold)) (<= (.x (Variables|Inertia|GetInertiaDirection)) (* -1.0 (.x _inertiatreshold))) (>= (.y (Variables|Inertia|GetInertiaDirection)) (.y _inertiatreshold)) (<= (.y (Variables|Inertia|GetInertiaDirection)) (* -1.0 (.y _inertiatreshold))))
        (Components|Timeline|ReversefromEnd (Variables|Default|GetMapRotationInertia)))
      (Variables|Map|SetMapRotation false))
    (:else)))

(fn ConfirmationButtonPressed
  (bind _campselected (Variables|Map|GetCampSelected))
  (Default|MapPanelCheckStep (Variables|Default|GetTaskManager) (Variables|/Game/Blueprints/Panels/BP_Camp.BP_Camp_C|GetName _campselected) (Variables|/Game/Blueprints/Panels/BP_Camp.BP_Camp_C|GetState _campselected)))

(fn MapRotationReleased)