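; Player controller that turns single-finger touch into interactions with map tactics, call center, button panel, task, cuff and screw actors.
; On press, a trace reads the hit actor's first tag to cache the target and set an enum that routes press, move and release.
; Untagged hits rotate a selected screw or, in first person, start a timeline-limited camera swipe.
; A Dialogue timeline holds typewriter text logic for the player UI.
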(event EventBeginPlay
  ;[0.15 0.15 0.15 0.5] Set Begin Play
  (Components|Timeline|SetPlayRate (Variables|Default|GetDelaySwipeRotationCamera) (/ 1.0 (Variables|RotationCamera|GetDelayStopSwipeRotCam)))
  (Components|Timeline|SetPlayRate (Variables|Default|GetDialogue) (/ 1.0 (Variables|Dialogue|GetDialogueSpeed)))
  (bind _asbp_character (Utilities|Casting|CastToBP_Character (Game|Player|GetPlayerPawn 0)))
  (Variables|Default|SetPlayerCharacter _asbp_character))

(event Input|TouchEvents|InputTouch
  (params (Location :type Vector) (FingerIndex :type ETouchIndex%20Enum))
  (bind _hitresult (Class|PlayerController|GetHitResultUnderFingerbyChannel "Touch1" "TraceTypeQuery1" true))
  ;[0.15 0.15 0.15 0.5] Touch Manager
  (:Pressed
    (switch Utilities|FlowControl|Switch|SwitchonETouchIndex FingerIndex
      (:Touch1
        ;;[0.15 0.15 0.15 0.5] Pressed
        (Variables|TouchPressed|SetStartTouchPosition (Math|Vector2D|MakeVector2D (.x Location) (.y Location)))
        (Variables|TouchPressed|SetHitComponent (.hitcomponent _hitresult))
        (Variables|TouchPressed|SetHitActor (.hitactor _hitresult))
        (CallFunction|VerifCastActor)
        (switch Utilities|FlowControl|Switch|SwitchonE_Actor (Variables|CastActor|GetEnumActor)
          (:NewEnumerator0
            ;;;[0.15 0.15 0.15 0.5] MapTactic Pressed
            (Default|MapTacticPressed (Variables|CastActor|GetMapTactics) (Variables|TouchPressed|GetHitComponent) (Variables|TouchPressed|GetStartTouchPosition)))
          (:NewEnumerator1
            ;;;[0.15 0.15 0.15 0.5] CallCenter Pressed
            (Default|CallCenterPressed (Variables|CastActor|GetCallCenter) (Variables|TouchPressed|GetStartTouchPosition) (Variables|TouchPressed|GetHitComponent)))
          (:NewEnumerator2
            ;;;[0.15 0.15 0.15 0.5] ButtonPanel Pressed
            (Default|ButtonPanelPressed (Variables|CastActor|GetButtonPanel) (Variables|TouchPressed|GetStartTouchPosition) (Variables|TouchPressed|GetHitComponent)))
          (:NewEnumerator4
            ;;;[0.15 0.15 0.15 0.5] Task
            (Default|OpenClose (Variables|CastActor|GetCurrentTask)))
          (:NewEnumerator7
            ;;;[0.15 0.15 0.15 0.5] Cuff
            (Default|CuffPressed (Variables|CastActor|GetCurrent%20Cuff)))))))
  (:Released
    (switch Utilities|FlowControl|Switch|SwitchonETouchIndex FingerIndex
      (:Touch1
        ;;[0.15 0.15 0.15 0.5] Released
        (switch Utilities|FlowControl|Switch|SwitchonE_Actor (Variables|CastActor|GetEnumActor)
          (:NewEnumerator0
            (Default|MapTacticReleased (Variables|CastActor|GetMapTactics) (Variables|TouchPressed|GetCurrentTouchPosition)))
          (:NewEnumerator1
            (Default|CallCenterReleased (Variables|CastActor|GetCallCenter)))
          (:NewEnumerator2
            (Default|ButtonPanelReleased (Variables|CastActor|GetButtonPanel)))
          (:NewEnumerator3
            (Variables|TouchPressed|SetIsTouchActive false))))))
  (:Moved
    (switch Utilities|FlowControl|Switch|SwitchonETouchIndex FingerIndex
      (:Touch1
        ;;[0.15 0.15 0.15 0.5] Move
        (Variables|TouchPressed|SetCurrentTouchPosition (Math|Vector2D|MakeVector2D (.x Location) (.y Location)))
        (switch Utilities|FlowControl|Switch|SwitchonE_Actor (Variables|CastActor|GetEnumActor)
          (:NewEnumerator0
            (Default|MapRotationFollow (Variables|CastActor|GetMapTactics) (Variables|TouchPressed|GetCurrentTouchPosition)))
          (:NewEnumerator1
            (Default|CableFollow (Variables|CastActor|GetCallCenter) (Variables|TouchPressed|GetCurrentTouchPosition)))
          (:NewEnumerator2
            (Default|SliderFollow (Variables|CastActor|GetButtonPanel) (Variables|TouchPressed|GetCurrentTouchPosition)))
          (:NewEnumerator3
            (RotationCamera|CameraRotationMove))
          (:NewEnumerator5
            (Default|ScrewRotationFollow (Variables|CastActor|GetCurrentScrew) (Variables|TouchPressed|GetCurrentTouchPosition) :!label _label))
          (:NewEnumerator8
            (goto _label)))))))

(fn ConstructionScript)

(fn CameraRotationPressed
  (Variables|RotationCamera|SetFirstPointerLocation (.x (Variables|TouchPressed|GetStartTouchPosition)))
  (Variables|TouchPressed|SetIsTouchActive true)
  ;[0.15 0.15 0.15 0.5] Makes sure it's a swipe (cancels itself on drag)
  (Components|Timeline|PlayfromStart (Variables|Default|GetDelaySwipeRotationCamera)))

(fn CameraRotationMove
  (bind _output_get (Variables|RotationCamera|SetCurrentPointerLocation (.x (Variables|TouchPressed|GetCurrentTouchPosition))))
  (if (Variables|TouchPressed|GetIsTouchActive)
    (Utilities|FlowControl|Sequence
      (:then_0
        (if (> (- (Variables|RotationCamera|GetFirstPointerLocation) _output_get) (Variables|RotationCamera|GetMovementTreshold))
          (bind _asbp_character (Utilities|Casting|CastToBP_Character (Game|Player|GetPlayerPawn 0)))
          (Default|RotateCameratoRight _asbp_character)
          (Variables|TouchPressed|SetIsTouchActive false)))
      (:then_1
        (if (< (- (Variables|RotationCamera|GetFirstPointerLocation) _output_get) (* -1.0 (Variables|RotationCamera|GetMovementTreshold)))
          (bind _asbp_character_2 (Utilities|Casting|CastToBP_Character (Game|Player|GetPlayerPawn 0)))
          (Default|RotateCameratoLeft _asbp_character_2)
          (Variables|TouchPressed|SetIsTouchActive false))))))

(fn VerifCastActor
  (switch name (Utilities|Array|Get(acopy) (Variables|/Script/Engine.Actor|GetTags (Variables|TouchPressed|GetHitActor)))
    (:Default
      ;[0.15 0.15 0.15 0.5] POV Context Dependants
      (if (Variables|/Game/Blueprints/Player/BP_Character.BP_Character_C|GetIsInFirstPerson (Variables|Default|GetPlayerCharacter))
        ;;[0.15 0.15 0.15 0.5] Camera Rotation
        (RotationCamera|CameraRotationPressed)
        (Variables|CastActor|SetEnumActor "NewEnumerator3")
        (else
          ;;[0.15 0.15 0.15 0.5] When a screw is selected and the player tries to make it rotate
          (bind _currentscrew (Variables|CastActor|GetCurrentScrew)
            (:then
              (Default|ScrewPressed _currentscrew (Variables|TouchPressed|GetStartTouchPosition))
              (Variables|CastActor|SetEnumActor "NewEnumerator8"))
            (:else)))))
    (:MapTactic
      ;[0.15 0.15 0.15 0.5] Cast MapTactic
      (bind _asbp_map_tactics (Utilities|Casting|CastToBP_MapTactics (Variables|TouchPressed|GetHitActor)))
      (Variables|CastActor|SetMapTactics _asbp_map_tactics)
      (Variables|CastActor|SetEnumActor "NewEnumerator0"))
    (:ButtonPanel
      ;[0.15 0.15 0.15 0.5] Cast Button Panel
      (bind _asbp_button_panel (Utilities|Casting|CastToBP_ButtonPanel (Variables|TouchPressed|GetHitActor)))
      (Variables|CastActor|SetButtonPanel _asbp_button_panel)
      (Variables|CastActor|SetEnumActor "NewEnumerator2"))
    (:Task
      ;[0.15 0.15 0.15 0.5] Cast Task
      (bind _asbp_task (Utilities|Casting|CastToBP_Task (Variables|TouchPressed|GetHitActor)))
      (Variables|CastActor|SetCurrentTask _asbp_task)
      (Variables|CastActor|SetEnumActor "NewEnumerator4"))
    (:CallCenter
      ;[0.15 0.15 0.15 0.5] CallCenter Panel
      (bind _asbp_call_center (Utilities|Casting|CastToBP_CallCenter (Variables|TouchPressed|GetHitActor)))
      (Variables|CastActor|SetCallCenter _asbp_call_center)
      (Variables|CastActor|SetEnumActor "NewEnumerator1"))
    (:Screw
      ;[0.15 0.15 0.15 0.5] Escape Panel (inside Cuff blueprint)
      (bind _asbp_screw (Utilities|Casting|CastToBP_Screw (Variables|TouchPressed|GetHitActor)))
      (Variables|CastActor|SetCurrentScrew _asbp_screw)
      (Variables|CastActor|SetEnumActor "NewEnumerator5"))
    (:Cuff
      ;[0.15 0.15 0.15 0.5] Cuff
      (bind _asbp_cuff (Utilities|Casting|CastToBP_Cuff (Variables|TouchPressed|GetHitActor)))
      (Variables|CastActor|SetCurrent%20Cuff _asbp_cuff)
      (Variables|CastActor|SetEnumActor "NewEnumerator7"))))