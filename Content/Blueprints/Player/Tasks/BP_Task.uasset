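; BP_Task is a timed task actor with three checkable steps, occupying a slot in a TaskManager.
; Initialize fills its widgets from target data and grays it out; Activate starts a timeline depleting the time bar and registers it as the active task.
; OpenClose toggles a short vertical slide via timeline.
; Completing all steps or running out of time frees the slot and destroys the actor; Error Gauge handling is only a print stub.
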(event EventBeginPlay
  (bind _output_get (Variables|Movement|SetBaseLocation (Transformation|GetActorLocation)))
  (Variables|Movement|SetTargetLocation (+ _output_get "0.000000,0.000000,11.000000"))
  (Components|Timeline|SetPlayRate (Variables|Default|GetOpenClose%20Timeline) (/ 1.0 (Variables|Movement|GetOpenCloseMovementSpeed)))
  (bind _returnvalue (UserInterface|CreateWidget "/Game/UI/InWorldUI/WBP_Task.WBP_Task_C"))
  (bind _output_get_2 (Variables|TopPart|SetTimeBarWidget _returnvalue))
  (UserInterface|SetWidget (Variables|Default|GetTimeGaugeWidget) _output_get_2)
  (bind _returnvalue_2 (UserInterface|CreateWidget "/Game/UI/InWorldUI/WBP_Task_CheckMarks.WBP_Task_CheckMarks_C"))
  (bind _output_get_3 (Variables|BottomPart|SetCheckMarksWidget _returnvalue_2))
  (UserInterface|SetWidget (Variables|Default|GetCheckBoxesWidget) _output_get_3))

(fn ConstructionScript)

(fn Initialize
  (params (Target :type BP%20DA%20Task%20Data%20Object%20Reference) (TaskManager :type BP%20Task%20Manager%20Object%20Reference) (TaskPositionIndex :type Integer))
  (bind _checkmarkswidget (Variables|BottomPart|GetCheckMarksWidget))
  (Variables|ProgressionTracking|SetTaskManager TaskManager)
  (Variables|ProgressionTracking|SetTaskPositionIndex TaskPositionIndex)
  (Default|SetUpText _checkmarkswidget (Utilities|Text|ToText(String) (Variables|/Game/Blueprints/Player/Tasks/BP_DA_Task_Data.BP_DA_Task_Data_C|GetFirstTaskText Target)) (Utilities|Text|ToText(String) (Variables|/Game/Blueprints/Player/Tasks/BP_DA_Task_Data.BP_DA_Task_Data_C|GetSecondTaskText Target)) (Utilities|Text|ToText(String) (Variables|/Game/Blueprints/Player/Tasks/BP_DA_Task_Data.BP_DA_Task_Data_C|GetThirdTaskText Target)))
  (Default|SetUpImages _checkmarkswidget)
  (CallFunction|SetUpConditions (Variables|/Game/Blueprints/Player/Tasks/BP_DA_Task_Data.BP_DA_Task_Data_C|GetBase Target) (Variables|/Game/Blueprints/Player/Tasks/BP_DA_Task_Data.BP_DA_Task_Data_C|GetStatus Target))
  (bind _output_get (Variables|TopPart|SetTotalTime (Variables|/Game/Blueprints/Player/Tasks/BP_DA_Task_Data.BP_DA_Task_Data_C|GetTime Target)))
  (Variables|TopPart|SetRemainingTime _output_get)
  (CallFunction|GrayedOut))

(fn GrayedOut
  (Rendering|Material|SetMaterial (Variables|Default|GetPlane) 0 0)
  (Rendering|SetVisibility (Variables|Default|GetCheckBoxesWidget) false false)
  (Class|ProgressBar|SetFillColorandOpacity (Variables|/Game/UI/InWorldUI/WBP_Task.WBP_Task_C|GetTimeBar (Variables|TopPart|GetTimeBarWidget)) "(R=0.200000,G=0.200000,B=0.200000,A=1.000000)"))

(fn Activate
  ;[0.15 0.15 0.15 0.5] Task Gauge playspeed Setup
  (Components|Timeline|SetPlayRate (Variables|Default|GetTimeGaugeTimeline) (/ 1.0 (Variables|TopPart|GetTotalTime)))
  ;[0.15 0.15 0.15 0.5] Task Gauge Start Depleting
  (Components|Timeline|PlayfromStart (Variables|Default|GetTimeGaugeTimeline))
  ;[0.15 0.15 0.15 0.5] Visual Enabling
  (Rendering|Material|SetMaterial (Variables|Default|GetPlane) 0 0)
  (Rendering|SetVisibility (Variables|Default|GetCheckBoxesWidget) true false)
  (Class|ProgressBar|SetFillColorandOpacity (Variables|/Game/UI/InWorldUI/WBP_Task.WBP_Task_C|GetTimeBar (Variables|TopPart|GetTimeBarWidget)) "(R=0.045795,G=0.747826,B=0.000000,A=1.000000)")
  (Variables|/Game/Blueprints/Player/Tasks/BP_TaskManager.BP_TaskManager_C|SetIsAnyTaskActivated (Variables|ProgressionTracking|GetTaskManager) true)
  (Variables|/Game/Blueprints/Player/Tasks/BP_TaskManager.BP_TaskManager_C|SetCurrentActiveTask (Variables|ProgressionTracking|GetTaskManager) self))

(fn EndTask
  (bind _remainingtime (Variables|TopPart|GetRemainingTime))
  (bind _taskmanager (Variables|ProgressionTracking|GetTaskManager))
  (Audio|Components|Audio|Stop (Variables|Default|GetTimeGaugeTimeline))
  (Variables|/Game/Blueprints/Player/Tasks/BP_TaskManager.BP_TaskManager_C|SetIsAnyTaskActivated _taskmanager false)
  (Default|EmptyTaskSlot _taskmanager (Variables|ProgressionTracking|GetTaskPositionIndex))
  ;[0.15 0.15 0.15 0.5] Function to implement :
  ; Error Gauge augmentation (WIP)
  (if (> _remainingtime 0.0)
    (Development|PrintString (Utilities|String|ToString(Float) _remainingtime))
    (Development|PrintString "add to Error Gauge"))
  (Actor|DestroyActor))

(fn OpenClose
  (if (not (Variables|Movement|GetIsOpening))
    (if (Variables|Movement|GetIsOpened)
      (Components|Timeline|ReversefromEnd (Variables|Default|GetOpenClose%20Timeline))
      (Variables|Movement|SetIsOpening true)
      (Variables|Movement|SetIsOpened false)
      (else
        (Components|Timeline|PlayfromStart (Variables|Default|GetOpenClose%20Timeline))
        (Variables|Movement|SetIsOpening true)
        (Variables|Movement|SetIsOpened true)))))

(fn CheckStep
  (params (StepIndex :type Integer))
  (bind _stepscompleted (Variables|ProgressionTracking|GetStepsCompleted))
  (if (Variables|ProgressionTracking|GetHasStarted)
    ;[0.15 0.15 0.15 0.5] Update image
    (Rendering|SetVisibility (Variables|Default|GetCheckBoxesWidget) false false)
    (Default|SetXBrushtoChecked (Variables|BottomPart|GetCheckMarksWidget) StepIndex)
    (Rendering|SetVisibility (Variables|Default|GetCheckBoxesWidget) true false)
    ;[0.15 0.15 0.15 0.5] Update Steps completion status
    (Utilities|Array|SetArrayElem (Variables|ProgressionTracking|GetStepsCompleted) StepIndex true)
    ;[0.15 0.15 0.15 0.5] All steps completed ?
    (if (and (and (Utilities|Array|Get(acopy) _stepscompleted) (Utilities|Array|Get(acopy) _stepscompleted 1)) (Utilities|Array|Get(acopy) _stepscompleted 2))
      (CallFunction|EndTask))))

(fn SetUpConditions
  (params (BaseName :type E_BasesNames%20Enum :default "NewEnumerator0") (BaseStatus :type E_BasesStatuses%20Enum :default "NewEnumerator0"))
  (Variables|TacticalMapConditions|SetBaseName BaseName)
  (Variables|TacticalMapConditions|SetBaseStatus BaseStatus))