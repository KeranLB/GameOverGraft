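; Player controller that routes touch input to tagged interactive actors or turns it into camera-rotation swipes.
; On press, a cursor trace reads the hit actor's first tag and forwards to the map tactics, button panel or call center.
; An enum remembers that target for move and release, though the call center only receives presses.
; Other touches rotate BP_Character_M past a horizontal threshold, with a timeline intended to cancel slow drags.
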(event EventBeginPlay
  ;[0.15 0.15 0.15 0.5] Set Begin Play
  (Components|Timeline|SetPlayRate (Variables|Default|GetDelaySwipeRotationCamera) (/ 1.0 (Variables|RotationCamera|GetDelayStopSwipeRotCam))))

(event Input|TouchEvents|InputTouch
  (params (Location :type Vector) (FingerIndex :type ETouchIndex%20Enum))
  (bind _hitresult (Game|Player|GetHitResultUnderCursorbyChannel "TraceTypeQuery1" true))
  ;[0.15 0.15 0.15 0.5] Touch Manager
  (:Pressed
    (Variables|TouchPressed|SetStartTouchPosition (Math|Vector2D|MakeVector2D (.x Location) (.y Location)))
    (Variables|TouchPressed|SetHitComponent (.hitcomponent _hitresult))
    (Variables|TouchPressed|SetHitActor (.hitactor _hitresult))
    (CallFunction|VerifCastActor))
  (:Released
    (switch Utilities|FlowControl|Switch|SwitchonE_Actor (Variables|TouchPressed|GetEnumActor)
      (:NewEnumerator0
        (Default|MapTacticReleased (Variables|MapTacticPanel|GetMapTactics) (Variables|TouchPressed|GetCurrentTouchPosition)))
      (:NewEnumerator2
        (Default|ButtonPanelReleased (Variables|MapTacticPanel|GetButtonPanel)))
      (:NewEnumerator3
        (Variables|TouchPressed|SetIsTouchActive false))))
  (:Moved
    (Variables|TouchPressed|SetCurrentTouchPosition (Math|Vector2D|MakeVector2D (.x Location) (.y Location)))
    (switch Utilities|FlowControl|Switch|SwitchonE_Actor (Variables|TouchPressed|GetEnumActor)
      (:NewEnumerator0
        (Default|MapRotationFollow (Variables|MapTacticPanel|GetMapTactics) (Variables|TouchPressed|GetCurrentTouchPosition)))
      (:NewEnumerator2
        (Default|SliderFollow (Variables|MapTacticPanel|GetButtonPanel) (Variables|TouchPressed|GetCurrentTouchPosition)))
      (:NewEnumerator3
        (RotationCamera|CameraRotationMove)))))

(fn ConstructionScript)

(fn CameraRotationPressed
  (Variables|RotationCamera|SetFirstPointerLocation (.x (Variables|TouchPressed|GetStartTouchPosition)))
  (Variables|TouchPressed|SetIsTouchActive true)
  ;[0.15 0.15 0.15 0.5] Makes sure it's a swipe (cancels itself on drag)
  (Components|Timeline|PlayfromStart (Variables|Default|GetDelaySwipeRotationCamera)))

(fn CameraRotationMove
  (bind _output_get (Variables|RotationCamera|SetCurrentPointerLocation (.x (Variables|TouchPressed|GetCurrentTouchPosition))))
  (if (Variables|TouchPressed|GetIsTouchActive)
    (Utilities|FlowControl|Sequence
      (:then_0
        (if (> (- (Variables|RotationCamera|GetFirstPointerLocation) _output_get) (Variables|RotationCamera|GetMovementTreshold))
          (bind _asbp_character_m (Utilities|Casting|CastToBP_Character_M (Game|Player|GetPlayerPawn 0)))
          (Default|RotateCameratoRight _asbp_character_m)
          (Variables|TouchPressed|SetIsTouchActive false)))
      (:then_1
        (if (< (- (Variables|RotationCamera|GetFirstPointerLocation) _output_get) (* -1.0 (Variables|RotationCamera|GetMovementTreshold)))
          (bind _asbp_character_m_2 (Utilities|Casting|CastToBP_Character_M (Game|Player|GetPlayerPawn 0)))
          (Default|RotateCameratoLeft _asbp_character_m_2)
          (Variables|TouchPressed|SetIsTouchActive false))))))

(fn VerifCastActor
  (switch name (Utilities|Array|Get(acopy) (Variables|/Script/Engine.Actor|GetTags (Variables|TouchPressed|GetHitActor)))
    (:Default
      ;[0.15 0.15 0.15 0.5] Camera Rotation
      (RotationCamera|CameraRotationPressed)
      (Variables|TouchPressed|SetEnumActor "NewEnumerator3")
      (Development|PrintString "Can Swipe"))
    (:MapTactic
      ;[0.15 0.15 0.15 0.5] Cast MapTactic
      (bind _asbp_map_tactics (Utilities|Casting|CastToBP_MapTactics (Variables|TouchPressed|GetHitActor)))
      (bind _output_get (Variables|MapTacticPanel|SetMapTactics _asbp_map_tactics))
      (Default|MapTacticPressed _output_get (Variables|TouchPressed|GetHitComponent) (Variables|TouchPressed|GetStartTouchPosition))
      (Variables|TouchPressed|SetEnumActor "NewEnumerator0")
      (Development|PrintString "MapTactic"))
    (:ButtonPanel
      ;[0.15 0.15 0.15 0.5] Cast Button Panel
      (bind _asbp_button_panel (Utilities|Casting|CastToBP_ButtonPanel (Variables|TouchPressed|GetHitActor)))
      (bind _output_get_2 (Variables|MapTacticPanel|SetButtonPanel _asbp_button_panel))
      (Default|ButtonPanelPressed _output_get_2 (Variables|TouchPressed|GetStartTouchPosition) (Variables|TouchPressed|GetHitComponent))
      (Variables|TouchPressed|SetEnumActor "NewEnumerator2")
      (Development|PrintString "ButtonPanel"))
    (:CallCenter
      ;[0.15 0.15 0.15 0.5] CallCenter Panel
      (bind _asbp_call_center (Utilities|Casting|CastToBP_CallCenter (Variables|TouchPressed|GetHitActor)))
      (bind _output_get_3 (Variables|MapTacticPanel|SetCallCenter _asbp_call_center))
      (Default|CallCenterPressed _output_get_3 (Variables|TouchPressed|GetStartTouchPosition) (Variables|TouchPressed|GetHitComponent))
      (Variables|TouchPressed|SetEnumActor "NewEnumerator1")
      (Development|PrintString "CallCenter"))
    (:Escape)))