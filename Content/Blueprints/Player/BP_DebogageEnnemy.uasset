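; Debug Blueprint for testing how an enemy's State Tree responds to logic control and events.
; Left, center and right check events each send the TestErreur event to the Enemy State Tree and print which check fired.
; They differ in logic handling: left restarts before sending, center stops, sends, then starts, and right stops without restarting.
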(event Custom|KeftCheck
  (bind _enemy (Variables|Default|GetEnemy))
  (Class|BrainComponent|RestartLogic _enemy)
  (Gameplay|StateTree|SendStateTreeEvent _enemy (Variables|Default|GetTestErreur) :!class /Script/GameplayStateTreeModule.StateTreeComponent)
  (Development|PrintString "Left check"))

(event Custom|CenterCheck
  (AI|Logic|StopLogic (Variables|Default|GetEnemy) "")
  (Gameplay|StateTree|SendStateTreeEvent (Variables|Default|GetEnemy) (Variables|Default|GetTestErreur) :!class /Script/GameplayStateTreeModule.StateTreeComponent)
  (AI|Logic|StartLogic (Variables|Default|GetEnemy))
  (Development|PrintString "Center check"))

(event Custom|RightCheck
  (AI|Logic|StopLogic (Variables|Default|GetEnemy) "")
  (Gameplay|StateTree|SendStateTreeEvent (Variables|Default|GetEnemy) (Variables|Default|GetTestErreur) :!class /Script/GameplayStateTreeModule.StateTreeComponent)
  (Development|PrintString "Right Check"))

(event EventBeginPlay)

(event EventTick
  (params (DeltaSeconds :type Float%20%28single-precision%29)))