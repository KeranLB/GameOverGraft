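; Player character that switches between third-person and first-person views behind a blink transition and wins by freeing all its cuffs.
; A timeline drives UI eyelid sliders, swapping cameras while closed, while another lerps the first-person camera between three anchors with shakes.
; A heartbeat timeline feeds the heart widget, its rate mapped from a supplied distance.
; Victory reuses the dead flag to blink to the death camera, then load the menu.
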(event Custom|ChangeView
  ;[0.15 0.15 0.15 0.5] 1ST/3RD Swap
  (Variables|Default|GetIsDead
    (:then
      (Components|Activation|SetActive (Variables|Default|GetCamera1stView) false false)
      (Components|Activation|SetActive (Variables|Default|GetCamera3dView) false false)
      (Components|Activation|SetActive (Variables|Default|GetCameraDeadView) true false)
      (Utilities|FlowControl|Delay 2.0)
      (CallFunction|GoBacktoMenu))
    (:else
      (if (Variables|Camera|GetIsInFirstPerson)
        (Components|Activation|SetActive (Variables|Default|GetCamera3dView) true false)
        (Components|Activation|SetActive (Variables|Default|GetCamera1stView) false false)
        (Variables|Camera|SetIsInFirstPerson false)
        (else
          (Components|Activation|SetActive (Variables|Default|GetCamera1stView) true false)
          (Components|Activation|SetActive (Variables|Default|GetCamera3dView) false false)
          (Variables|Camera|SetIsInFirstPerson true)))
      (Components|Timeline|ReversefromEnd (Variables|Default|GetBlinkTimeline)))))

(event Custom|RotateCameraToLeft
  ;[0.15 0.15 0.15 0.5] 1ST Person Camera Movement
  (if (Variables|Camera|GetIsInFirstPerson)
    (if (> (Variables|Camera|GetCameraPosition) 0)
      (CallFunction|LerpCamera -1)
      (else
        (bind _asbp_controller (Utilities|Casting|CastToBP_Controller (Pawn|GetController)))
        (Game|Feedback|ClientStartCameraShake _asbp_controller "/Game/UI/FirstPersonUI/CamShake_FirstPersonRotation.CamShake_FirstPersonRotation_C" 1.0 "CameraLocal" "0, 0, 0")))))

(event Custom|RotateCameraToRight
  ;[0.15 0.15 0.15 0.5] 1ST Person Camera Movement
  (if (Variables|Camera|GetIsInFirstPerson)
    (if (< (Variables|Camera|GetCameraPosition) 2)
      (CallFunction|LerpCamera 1)
      (else
        (bind _asbp_controller (Utilities|Casting|CastToBP_Controller (Pawn|GetController)))
        (Game|Feedback|ClientStartCameraShake _asbp_controller "/Game/UI/FirstPersonUI/CamShake_FirstPersonRotation.CamShake_FirstPersonRotation_C" 1.0 "CameraLocal" "0, 0, 0")))))

(event Custom|LerpCamera
  (params (TargetTransformIndex :type Integer))
  ;[0.15 0.15 0.15 0.5] 1ST Person Camera Movement
  (bind _newtrack_0 (Timeline|CameraRotation PlayFromStart)
    (:Update
      (Transformation|SetWorldLocationAndRotation (Variables|Default|GetCamera1stView) (.location (Math|Transform|Lerp(Transform) (Transformation|GetWorldTransform (Utilities|Array|Get(acopy) (Variables|Camera|GetTransformsCam) (Variables|Camera|GetCameraPosition))) (Transformation|GetWorldTransform (Utilities|Array|Get(acopy) (Variables|Camera|GetTransformsCam) (+ TargetTransformIndex (Variables|Camera|GetCameraPosition)))) _newtrack_0)) (.rotation (Math|Transform|Lerp(Transform) (Transformation|GetWorldTransform (Utilities|Array|Get(acopy) (Variables|Camera|GetTransformsCam) (Variables|Camera|GetCameraPosition))) (Transformation|GetWorldTransform (Utilities|Array|Get(acopy) (Variables|Camera|GetTransformsCam) (+ TargetTransformIndex (Variables|Camera|GetCameraPosition)))) _newtrack_0)) false false))
    (:Finished
      (bind _asbp_controller (Utilities|Casting|CastToBP_Controller (Pawn|GetController)))
      (Game|Feedback|ClientStartCameraShake _asbp_controller "/Game/UI/FirstPersonUI/CamShake_FirstPersonRotation.CamShake_FirstPersonRotation_C" 1.0 "CameraLocal" "0, 0, 0")
      (Variables|Camera|SetCameraPosition (+ (Variables|Camera|GetCameraPosition) TargetTransformIndex)))))

(event Custom|BlinkIN
  ;[0.15 0.15 0.15 0.5] 1ST/3RD Swap
  (Widget|SetVisibility (Variables|/Game/UI/FirstPersonUI/WBP_UI_Player.WBP_UI_Player_C|GetBottomSlider (Variables|Default|GetPlayerUI)) "Visible")
  (Widget|SetVisibility (Variables|/Game/UI/FirstPersonUI/WBP_UI_Player.WBP_UI_Player_C|GetTopSlider (Variables|Default|GetPlayerUI)) "Visible")
  (Variables|Camera|SetIsBlinking true)
  (bind _blinkin (Timeline|BlinkTimeline PlayFromStart)
    (:Update
      (Progress|SetPercent (Variables|/Game/UI/FirstPersonUI/WBP_UI_Player.WBP_UI_Player_C|GetTopSlider (Variables|Default|GetPlayerUI)) _blinkin)
      (Progress|SetPercent (Variables|/Game/UI/FirstPersonUI/WBP_UI_Player.WBP_UI_Player_C|GetBottomSlider (Variables|Default|GetPlayerUI)) _blinkin))
    (:Finished
      (if (Variables|Camera|GetIsBlinking)
        (Variables|Camera|SetIsBlinking false)
        (CallFunction|ChangeView)
        (else
          (Widget|SetVisibility (Variables|/Game/UI/FirstPersonUI/WBP_UI_Player.WBP_UI_Player_C|GetBottomSlider (Variables|Default|GetPlayerUI)) "Hidden")
          (Widget|SetVisibility (Variables|/Game/UI/FirstPersonUI/WBP_UI_Player.WBP_UI_Player_C|GetTopSlider (Variables|Default|GetPlayerUI)) "Hidden"))))))

(event Custom|UpdateBpm
  (params (Distance :type Float%20%28double-precision%29))
  ;[0.15 0.15 0.15 0.5] BPM Manager
  ;;[0.15 0.15 0.15 0.5] Set play rate to accelerate or slow the bpm
  (Components|Timeline|SetPlayRate (Variables|Default|GetBpm) (/ 1.0 (Math|Float|MapRangeClamped Distance (Variables|AtomicParameters|GetSafeDistance) (Variables|AtomicParameters|GetCloseDistance) (Variables|HeartPulse|GetSlowerPlayRate) (Variables|HeartPulse|GetFasterPlayRate)))))

(event Custom|GoBackToMenu
  (Game|OpenLevel(byObjectReference) "/Game/Levels/Lvl_Menu.Lvl_Menu"))

(event EventBeginPlay
  (bind _bpm (Variables|Default|GetBpm))
  (bind _transformscam (Variables|Camera|GetTransformsCam))
  (bind _cameraposition (Variables|Camera|GetCameraPosition))
  (bind _output (Utilities|Array|Get(acopy) _transformscam _cameraposition))
  (bind _returnvalue (Transformation|GetWorldTransform _output))
  (Utilities|FlowControl|Sequence
    (:then_0
      (Components|Activation|SetActive (Variables|Default|GetCameraDeadView) false false)
      ;[0.15 0.15 0.15 0.5] UI Player
      (Components|Activation|SetActive (Variables|Default|GetCamera3dView) true false)
      (bind _returnvalue_2 (UserInterface|CreateWidget "/Game/UI/FirstPersonUI/WBP_UI_Player.WBP_UI_Player_C"))
      (bind _output_get (Variables|Default|SetPlayerUI _returnvalue_2))
      (UserInterface|Viewport|AddtoViewport _output_get 0)
      (Variables|/Game/UI/FirstPersonUI/WBP_UI_Player.WBP_UI_Player_C|SetCharacter (Variables|Default|GetPlayerUI) self)
      (bind _returnvalue_3 (UserInterface|CreateWidget "/Game/UI/FirstPersonUI/WBP_Dialogue.WBP_Dialogue_C"))
      (Variables|UI|SetDialogueUI _returnvalue_3)
      ;[0.15 0.15 0.15 0.5] Set the 3 positions of the 1st view Camera
      (Utilities|Array|SetArrayElem (Variables|Camera|GetTransformsCam) 0 (Variables|Default|GetEmptyTaget_0))
      (Utilities|Array|SetArrayElem (Variables|Camera|GetTransformsCam) 1 (Variables|Default|GetEmptyTaget_1))
      (Utilities|Array|SetArrayElem (Variables|Camera|GetTransformsCam) 2 (Variables|Default|GetEmptyTaget_2))
      ;[0.15 0.15 0.15 0.5] Cuff List setup
      (bind _asbp_cuff (Utilities|Casting|CastToBP_Cuff (Variables|/Script/Engine.ChildActorComponent|GetChildActor (Variables|Default|GetCuff_1))))
      (Utilities|Array|Add (Variables|Default|GetCuffList) _asbp_cuff)
      (bind _asbp_cuff_2 (Utilities|Casting|CastToBP_Cuff (Variables|/Script/Engine.ChildActorComponent|GetChildActor (Variables|Default|GetCuff_2))))
      (Utilities|Array|Add (Variables|Default|GetCuffList) _asbp_cuff_2))
    (:then_1
      ;[0.15 0.15 0.15 0.5] Camera Rotation Speed
      (Components|Timeline|SetPlayRate (Variables|Default|GetCameraRotation) (/ 1.0 (Variables|AtomicParameters|GetRotationSpeed)))
      ;[0.15 0.15 0.15 0.5] Blink Speed
      (Components|Timeline|SetPlayRate (Variables|Default|GetBlinkTimeline) (/ 1.0 (Variables|Camera|GetBlinkSpeed)))
      ;[0.15 0.15 0.15 0.5] Set 1st view camera to the panel view
      (Transformation|SetWorldLocationAndRotation (Variables|Default|GetCamera1stView) (.location _returnvalue) (.rotation _returnvalue) false false)
      ;[0.15 0.15 0.15 0.5] Set Setings for bpm
      (Components|Timeline|SetPlayRate _bpm (/ 1.0 (Variables|HeartPulse|GetSlowerPlayRate)))
      (Components|Timeline|PlayfromStart _bpm)
      (UserInterface|CreateWidget "/Game/UI/FirstPersonUI/WBP_Bpm.WBP_Bpm_C")
      (bind _aswbp_bpm (Utilities|Casting|CastToWBP_Bpm (UserInterface|GetWidget (Variables|Default|GetUI_Hearth))))
      (Variables|UI|SetHeartUI _aswbp_bpm))))

(fn ConstructionScript)

(fn CheckWinConditions
  (Variables|Default|SetCheckIsFree true)
  (bind _array_element (Utilities|Array|ForEachLoopwithBreak (Variables|Default|GetCuffList))
    (:LoopBody
      (if (not (Variables|/Game/Blueprints/Panels/BP_Cuff.BP_Cuff_C|GetIsFree _array_element))
        (Variables|Default|SetCheckIsFree false)))
    (:Completed
      (Variables|Default|GetCheckIsFree
        (:then
          ;[0.15 0.15 0.15 0.5] Put Winning logic here
          (Development|PrintString "VICTORY!")
          (Variables|Default|SetIsDead true)
          (CallFunction|BlinkIN))
        (:else)))))