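; Player character that swaps between third- and first-person cameras and creates its player UI widget on BeginPlay.
; The view swap hides behind an eye blink: a timeline closes the widget's top and bottom sliders, toggles the active camera, then reverses to reopen.
; In first person, left/right events step the camera through three positions by timeline-lerping location and yaw, with camera shake on arrival or at either limit.
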(event Custom|ChangeView
  ;[0.15 0.15 0.15 0.5] 1ST/3RD Swap
  (if (Variables|Default|GetIsInFirstPerson)
    (Components|Activation|SetActive (Variables|Default|GetCamera3dView) true false)
    (Components|Activation|SetActive (Variables|Default|GetCamera1stView) false false)
    (Variables|Default|SetIsInFirstPerson false)
    (else
      (Components|Activation|SetActive (Variables|Default|GetCamera1stView) true false)
      (Components|Activation|SetActive (Variables|Default|GetCamera3dView) false false)
      (Variables|Default|SetIsInFirstPerson true)))
  (Components|Timeline|ReversefromEnd (Variables|Default|GetTimeline_0)))

(event Custom|RotateCameraToLeft
  ;[0.15 0.15 0.15 0.5] 1ST Person Camera Movement
  (if (Variables|Default|GetIsInFirstPerson)
    (if (> (Variables|Default|GetCameraPosition) 0)
      (if (== (- (Variables|Default|GetCameraPosition) 1) 1)
        (bind _output_get (Variables|Default|SetTargetCameraLocationY 5e+01))
        (CallFunction|NewLerpRotation 2e+01 _output_get 45.0)
        (Variables|Default|SetCameraPosition (- (Variables|Default|GetCameraPosition) 1))
        (else
          (bind _output_get_2 (Variables|Default|SetTargetCameraLocationY -5e+01))
          (CallFunction|NewLerpRotation -2e+01 _output_get_2 45.0)
          (Variables|Default|SetCameraPosition (- (Variables|Default|GetCameraPosition) 1))))
      (else
        (bind _asbp_controller_m (Utilities|Casting|CastToBP_Controller_M (Pawn|GetController)))
        (Game|Feedback|ClientStartCameraShake _asbp_controller_m "/Game/UI/FirstPersonUI/CamShake_FirstPersonRotation.CamShake_FirstPersonRotation_C" 1.0 "CameraLocal" "0, 0, 0")))))

(event Custom|RotateCameraToRight
  ;[0.15 0.15 0.15 0.5] 1ST Person Camera Movement
  (if (Variables|Default|GetIsInFirstPerson)
    (if (< (Variables|Default|GetCameraPosition) 2)
      (if (== (+ (Variables|Default|GetCameraPosition) 1) 1)
        (bind _output_get (Variables|Default|SetTargetCameraLocationY 5e+01))
        (CallFunction|NewLerpRotation -2e+01 _output_get -45.0)
        (Variables|Default|SetCameraPosition (+ (Variables|Default|GetCameraPosition) 1))
        (else
          (bind _output_get_2 (Variables|Default|SetTargetCameraLocationY -5e+01))
          (CallFunction|NewLerpRotation -2e+01 _output_get_2 -45.0)
          (Variables|Default|SetCameraPosition (+ (Variables|Default|GetCameraPosition) 1))))
      (else
        (bind _asbp_controller_m (Utilities|Casting|CastToBP_Controller_M (Pawn|GetController)))
        (Game|Feedback|ClientStartCameraShake _asbp_controller_m "/Game/UI/FirstPersonUI/CamShake_FirstPersonRotation.CamShake_FirstPersonRotation_C" 1.0 "CameraLocal" "0, 0, 0")))))

(event Custom|LerpCamera
  (params (TargetTransformIndex :type Integer))
  ;[0.15 0.15 0.15 0.5] 1ST Person Camera Movement
  (Variables|Default|SetStartRotation (Transformation|GetActorLocation)))

(event Custom|BlinkIN
  ;[0.15 0.15 0.15 0.5] 1ST/3RD Swap
  (Widget|SetVisibility (Variables|/Game/UI/FirstPersonUI/WBP_UI_Player_K.WBP_UI_Player_K_C|GetBottomSlider (Variables|Default|GetWidgetUI)) "Visible")
  (Widget|SetVisibility (Variables|/Game/UI/FirstPersonUI/WBP_UI_Player_K.WBP_UI_Player_K_C|GetTopSlider (Variables|Default|GetWidgetUI)) "Visible")
  (Variables|Default|SetIsBlinking true)
  (bind _blinkin (Timeline|Timeline_0 PlayFromStart)
    (:Update
      (Progress|SetPercent (Variables|/Game/UI/FirstPersonUI/WBP_UI_Player_K.WBP_UI_Player_K_C|GetTopSlider (Variables|Default|GetWidgetUI)) _blinkin)
      (Progress|SetPercent (Variables|/Game/UI/FirstPersonUI/WBP_UI_Player_K.WBP_UI_Player_K_C|GetBottomSlider (Variables|Default|GetWidgetUI)) _blinkin))
    (:Finished
      (if (Variables|Default|GetIsBlinking)
        (Variables|Default|SetIsBlinking false)
        (CallFunction|ChangeView)
        (else
          (Widget|SetVisibility (Variables|/Game/UI/FirstPersonUI/WBP_UI_Player_K.WBP_UI_Player_K_C|GetBottomSlider (Variables|Default|GetWidgetUI)) "Hidden")
          (Widget|SetVisibility (Variables|/Game/UI/FirstPersonUI/WBP_UI_Player_K.WBP_UI_Player_K_C|GetTopSlider (Variables|Default|GetWidgetUI)) "Hidden"))))))

(event Custom|NewLerpRotation
  (params (LocationX :type Float%20%28double-precision%29) (LocationY :type Float%20%28double-precision%29) (RotationZ :type Float%20%28double-precision%29))
  (bind _camera1stview (Variables|Default|GetCamera1stView))
  (bind _camera1stview_2 (Variables|Default|GetCamera1stView))
  (bind _returnvalue (Transformation|GetWorldLocation _camera1stview))
  (bind _returnvalue_2 (Transformation|GetWorldRotation _camera1stview))
  (bind _returnvalue_3 (Transformation|GetWorldRotation _camera1stview_2))
  (Variables|Default|SetVectorSafeStartlocandrota (Math|Vector|MakeVector (.x _returnvalue) (.y _returnvalue) (.yaw _returnvalue_2)))
  (Variables|Default|SetVectorSafeTargetlocandrota_0 (Math|Vector|MakeVector (+ (.x _returnvalue) LocationX) (+ (.y _returnvalue) LocationY) (+ (.yaw _returnvalue_2) RotationZ)))
  (bind _newtrack_0 (Timeline|CameraRotation PlayFromStart)
    (:Update
      (Transformation|SetWorldLocationAndRotation (Variables|Default|GetCamera1stView) (Math|Vector|MakeVector (Math|Float|Lerp (.x (Variables|Default|GetVectorSafeStartlocandrota)) (.x (Variables|Default|GetVectorSafeTargetlocandrota_0)) _newtrack_0) (Math|Float|Lerp (.y (Variables|Default|GetVectorSafeStartlocandrota)) (.y (Variables|Default|GetVectorSafeTargetlocandrota_0)) _newtrack_0) (.z (Transformation|GetWorldLocation _camera1stview_2))) (Math|Rotator|MakeRotator (.roll _returnvalue_3) (.pitch _returnvalue_3) (Math|Float|Lerp (.z (Variables|Default|GetVectorSafeStartlocandrota)) (.z (Variables|Default|GetVectorSafeTargetlocandrota_0)) _newtrack_0)) false false))
    (:Finished
      (bind _asbp_controller (Utilities|Casting|CastToBP_Controller (Pawn|GetController)))
      (Game|Feedback|ClientStartCameraShake _asbp_controller "/Game/UI/FirstPersonUI/CamShake_FirstPersonRotation.CamShake_FirstPersonRotation_C" 1.0 "CameraLocal" "0, 0, 0"))))

(event EventBeginPlay
  (Utilities|FlowControl|Sequence
    (:then_0
      ;[0.15 0.15 0.15 0.5] UI Player
      (Components|Activation|SetActive (Variables|Default|GetCamera3dView) true false)
      (bind _returnvalue (UserInterface|CreateWidget "/Game/UI/FirstPersonUI/WBP_UI_Player_K.WBP_UI_Player_K_C"))
      (bind _output_get (Variables|Default|SetWidgetUI _returnvalue))
      (UserInterface|Viewport|AddtoViewport _output_get 0)
      (Variables|/Game/UI/FirstPersonUI/WBP_UI_Player_K.WBP_UI_Player_K_C|SetCharacter (Variables|Default|GetWidgetUI) self))
    (:then_1
      ;[0.15 0.15 0.15 0.5] Camera Rotation Speed
      (Components|Timeline|SetPlayRate (Variables|Default|GetCameraRotation) (/ 1.0 (Variables|Default|GetRotationSpeed)))
      ;[0.15 0.15 0.15 0.5] Blink Speed
      (Components|Timeline|SetPlayRate (Variables|Default|GetTimeline_0) (/ 1.0 (Variables|Default|GetBlinkSpeed))))))

(fn ConstructionScript)