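; BP_Escape is an unfinished player Blueprint for a touch-driven escape control with Screw and Rotator components.
; EscapePressed stores the starting touch position and EscapeRotationFollow stores the current one, but no logic uses either.
; A disconnected "Follow target" chain would pitch Screw toward Rotator with FindLookAtRotation and RInterpTo, preserving roll and yaw.
; The event graph's events are empty, so nothing rotates at runtime.
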(event EventBeginPlay)

(event Collision|EventActorBeginOverlap
  (params (OtherActor :type Actor%20Object%20Reference)))

(event EventTick
  (params (DeltaSeconds :type Float%20%28single-precision%29)))

(fn ConstructionScript)

(fn EscapePressed
  (params (StartPosition :type Vector%202D%20Structure))
  (Variables|Default|SetStartTouchPos StartPosition))

(fn EscapeRotationFollow
  (params (Touch%20Pos :type Vector%202D%20Structure))
  (Variables|Default|SetCurrentTouchPos Touch%20Pos))