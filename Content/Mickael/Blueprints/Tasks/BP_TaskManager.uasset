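; BP_TaskManager is an actor that spawns BP_Task actors into a set of position slots around itself.
; SpawnTask fills the first free slot, initializes the task with a random DataList entry, then removes that entry to prevent duplicates.
; TaskSpawnerTimeline acts as a repeating timer, with play rate scaled by TaskSpawnTime, restarted after every spawn attempt.
; EmptyTaskSlot frees a slot for reuse and clears the current active task.
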(event EventBeginPlay
  (CallFunction|SpawnTask)
  (Components|Timeline|SetPlayRate (Variables|Default|GetTaskSpawnerTimeline) (/ 1.0 (Variables|Spawning|GetTaskSpawnTime))))

(fn ConstructionScript)

(fn SpawnTask
  (bind _returnvalue (Transformation|GetActorTransform))
  (bind (_array_element _array_index) (Utilities|Array|ForEachLoopwithBreak (Variables|Spawning|GetIsPositionTaken) :!label _label)
    (:LoopBody
      ;[0.15 0.15 0.15 0.5] Spawns the task actor in a free position
      (if (not _array_element)
        (bind _returnvalue_2 (Game|SpawnActorfromClass "/Game/Mickael/Blueprints/Tasks/BP_Task.BP_Task_C" (Math|Transform|MakeTransform (+ (Utilities|Array|Get(acopy) (Variables|Spawning|GetPositions) _array_index) (.location _returnvalue)) (Math|Rotator|MakeRotator (.roll (.rotation _returnvalue)) (.pitch (.rotation _returnvalue)) (- (.yaw (.rotation _returnvalue)) 9e+01)) (.scale _returnvalue)) "Undefined" "MultiplyWithRoot" 0 0))
        ;[0.15 0.15 0.15 0.5] Takes a random index (task data) and removes it from the list. Prevents dupplicates.
        (LocalVariables|SetIndexToRemove (Math|Random|RandomInteger (Utilities|Array|Length (Variables|Spawning|GetDataList))))
        (Default|Initialize _returnvalue_2 (Utilities|Array|Get(acopy) (Variables|Spawning|GetDataList) (LocalVariables|GetIndexToRemove)) self _array_index)
        (Utilities|Array|RemoveIndex (Variables|Spawning|GetDataList) (LocalVariables|GetIndexToRemove))
        ;[0.15 0.15 0.15 0.5] Marks the slot as unavailable
        (Utilities|Array|SetArrayElem (Variables|Spawning|GetIsPositionTaken) _array_index true)
        (goto _label Break)))
    (:Completed
      ;[0.15 0.15 0.15 0.5] Loops again for another try in {TaskSpawnTime} seconds
      (Components|Timeline|PlayfromStart (Variables|Default|GetTaskSpawnerTimeline)))))

(fn EmptyTaskSlot
  (params (Index :type Integer))
  ;[0.15 0.15 0.15 0.5] Makes the slot available for new tasks
  (Utilities|Array|SetArrayElem (Variables|Spawning|GetIsPositionTaken) Index false)
  (Variables|ProgressTracking|SetCurrentActiveTask 0))