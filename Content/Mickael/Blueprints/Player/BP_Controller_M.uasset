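; Player controller that routes touch input to camera swipes, tactic map interaction or tasks, based on the tag of the component hit under the cursor.
; Horizontal swipes past a threshold rotate the character's camera left or right, with a timeline intended to reject slow drags.
; Map touches call BP_MapTactics to interact and rotate.
; Task touches open, close or activate tasks depending on whether one is already active; SpaceBar test-checks a step.
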(event EventBeginPlay
  (Variables|Default|SetbShowMouseCursor true)
  (Components|Timeline|SetPlayRate (Variables|Default|GetDelaySwipeRotationCamera) (/ 1.0 (Variables|RotationCamera|GetDelayStopSwipeRotCam))))

(event Input|KeyboardEvents|SpaceBar
  (params (Key :type Key%20Structure :default "None"))
  ;[0.15 0.15 0.15 0.5] Step Check Test
  (:Pressed
    (bind _currenttask (Variables|Task|GetCurrentTask)
      (:then
        (Default|CheckStep _currenttask))
      (:else
        (Development|PrintString "not valid")))))

(event Input|TouchEvents|InputTouch
  (params (Location :type Vector) (FingerIndex :type ETouchIndex%20Enum))
  (bind _hitresult (Game|Player|GetHitResultUnderCursorbyChannel "TraceTypeQuery1" true))
  (:Pressed
    (Variables|TouchPressed|SetStartTouchPosition (Math|Vector2D|MakeVector2D (.x Location) (.y Location)))
    (bind _output_get (Variables|TouchPressed|SetHitComponent (.hitcomponent _hitresult)))
    (Variables|TouchPressed|SetHitActor (.hitactor _hitresult))
    (CallFunction|VerifCastActor _output_get)
    (switch Utilities|FlowControl|Switch|SwitchonE_Actor (Variables|TouchPressed|GetEnumAction)
      (:NewEnumerator0
        (MapTacticPanel|MapTacticPressed (Variables|TouchPressed|GetHitActor) (Variables|TouchPressed|GetHitComponent)))
      (:NewEnumerator3
        (RotationCamera|CameraRotationPressed))
      (:NewEnumerator4
        ;[0.15 0.15 0.15 0.5] Task System :
        ; Any active task disables the activation of other tasks.
        ; If a task is opened before activation : doesn't close it. (ergonomicly better)
        (if (Variables|/Game/Mickael/Blueprints/Tasks/BP_TaskManager.BP_TaskManager_C|GetIsAnyTaskActivated (Variables|/Game/Mickael/Blueprints/Tasks/BP_Task.BP_Task_C|GetTaskManager (Variables|Task|GetCurrentTask)))
          (Default|OpenClose (Variables|Task|GetCurrentTask))
          (else
            (if (Variables|/Game/Mickael/Blueprints/Tasks/BP_Task.BP_Task_C|GetIsOpened (Variables|Task|GetCurrentTask))
              _
              (else
                (Default|OpenClose (Variables|Task|GetCurrentTask))))
            (Default|Activate (Variables|Task|GetCurrentTask)))))))
  (:Released
    (switch Utilities|FlowControl|Switch|SwitchonE_Actor (Variables|TouchPressed|GetEnumAction)
      (:NewEnumerator0
        (Variables|MapTacticPanel|SetMapRotation false))
      (:NewEnumerator3
        (Variables|RotationCamera|SetIsTouchActive false))))
  (:Moved
    (Variables|Default|SetCurrentTouchPosition (Math|Vector2D|MakeVector2D (.x Location) (.y Location)))
    (switch Utilities|FlowControl|Switch|SwitchonE_Actor (Variables|TouchPressed|GetEnumAction)
      (:NewEnumerator0
        (MapTacticPanel|MapTacticMove))
      (:NewEnumerator3
        (RotationCamera|CameraRotationMove)))))

(fn ConstructionScript)

(fn CameraRotationPressed
  (Variables|RotationCamera|SetFirstPointerLocation (.x (Variables|TouchPressed|GetStartTouchPosition)))
  (Variables|RotationCamera|SetIsTouchActive true)
  ;[0.15 0.15 0.15 0.5] Makes sure it's a swipe (cancels itself on drag)
  (Components|Timeline|PlayfromStart (Variables|Default|GetDelaySwipeRotationCamera)))

(fn CameraRotationMove
  (bind _output_get (Variables|RotationCamera|SetCurrentPointerLocation (.x (Variables|Default|GetCurrentTouchPosition))))
  (if (Variables|RotationCamera|GetIsTouchActive)
    (Utilities|FlowControl|Sequence
      (:then_0
        (if (> (- (Variables|RotationCamera|GetFirstPointerLocation) _output_get) (Variables|RotationCamera|GetMovementTreshold))
          (bind _asbp_character_m (Utilities|Casting|CastToBP_Character_M (Game|Player|GetPlayerPawn 0)))
          (Default|RotateCameratoRight _asbp_character_m)
          (Variables|RotationCamera|SetIsTouchActive false)))
      (:then_1
        (if (< (- (Variables|RotationCamera|GetFirstPointerLocation) _output_get) (* -1.0 (Variables|RotationCamera|GetMovementTreshold)))
          (bind _asbp_character_m_2 (Utilities|Casting|CastToBP_Character_M (Game|Player|GetPlayerPawn 0)))
          (Default|RotateCameratoLeft _asbp_character_m_2)
          (Variables|RotationCamera|SetIsTouchActive false))))))

(fn MapTacticPressed
  (params (HitActor :type Actor%20Object%20Reference) (HitComponent :type Primitive%20Component%20Object%20Reference))
  (bind _returnvalue (Utilities|GetObjectName HitComponent))
  (bind _asbp_map_tactics (Utilities|Casting|CastToBP_MapTactics HitActor))
  (bind _output_get (Variables|MapTacticPanel|SetMapTactics _asbp_map_tactics))
  (Development|PrintString _returnvalue)
  (bind _maprotation (Default|Interact _output_get _returnvalue))
  (Variables|MapTacticPanel|SetMapRotation _maprotation))

(fn MapTacticMove
  (bind _currenttouchposition (Variables|Default|GetCurrentTouchPosition))
  (Variables|MapTacticPanel|GetMapRotation
    (:then
      (bind _newstartposition (Default|MapRotation (Variables|MapTacticPanel|GetMapTactics) (Variables|TouchPressed|GetStartTouchPosition) (Math|Vector2D|MakeVector2D (.x _currenttouchposition) (.y _currenttouchposition))))
      (Variables|TouchPressed|SetStartTouchPosition _newstartposition))
    (:else)))

(fn VerifCastActor
  (params (HitComponent :type Primitive%20Component%20Object%20Reference))
  (bind _output_get (LocalVariables|SetComponentHit HitComponent))
  (switch name (Utilities|Array|Get(acopy) (Variables|/Script/Engine.ActorComponent|GetComponentTags _output_get))
    (:Default
      (Variables|TouchPressed|SetCastSucced false)
      (Variables|TouchPressed|SetEnumAction "NewEnumerator3")
      (Development|PrintString "Can Swipe"))
    (:MapTactic
      (bind _asbp_map_tactics (Utilities|Casting|CastToBP_MapTactics (Variables|TouchPressed|GetHitActor)))
      (Variables|MapTacticPanel|SetMapTactics _asbp_map_tactics)
      (Variables|TouchPressed|SetEnumAction "NewEnumerator0")
      (Development|PrintString "MapTactic"))
    (:Task
      (bind _asbp_task (Utilities|Casting|CastToBP_Task (Variables|TouchPressed|GetHitActor)))
      (Variables|Task|SetCurrentTask _asbp_task)
      (Variables|TouchPressed|SetEnumAction "NewEnumerator4")
      (Development|PrintString "Task"))))