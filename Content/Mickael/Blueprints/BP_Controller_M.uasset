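; BP_Controller_M is a controller that shows the mouse cursor and turns horizontal touch swipes into camera rotation on BP_Character_M.
; A press records the start X and opens a 0.2-second window, which release also closes, so slow drags are ignored.
; Moves beyond MovementTreshold within that window call RotateCameraToRight for leftward swipes or RotateCameraToLeft for rightward ones, then end the swipe so it fires once.
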(event EventBeginPlay
  (Variables|Default|SetbShowMouseCursor true))

(event Input|TouchEvents|InputTouch
  (params (Location :type Vector) (FingerIndex :type ETouchIndex%20Enum))
  ;[0.15 0.15 0.15 0.5] Camera Rotation With Swipe
  (:Pressed
    (bind _output_get (Variables|Default|SetFirstPointerLocation (.x Location)))
    (Variables|Default|SetIsTouchActive true)
    ;;[0.15 0.15 0.15 0.5] Makes sure it's a swipe (cancels itself on drag)
    (Utilities|FlowControl|Delay 0.2)
    (Variables|Default|SetIsTouchActive false))
  (:Released
    (Variables|Default|SetIsTouchActive false))
  (:Moved
    (bind _output_get_2 (Variables|Default|SetCurrentPointerLocation (.x Location)))
    (if (Variables|Default|GetIsTouchActive)
      (Utilities|FlowControl|Sequence
        (:then_0
          (if (> (- _output_get _output_get_2) (Variables|Default|GetMovementTreshold))
            (bind _asbp_character_m (Utilities|Casting|CastToBP_Character_M (Game|Player|GetPlayerPawn 0)))
            (Default|RotateCameratoRight _asbp_character_m)
            (Variables|Default|SetIsTouchActive false)))
        (:then_1
          (if (< (- _output_get _output_get_2) (* -1.0 (Variables|Default|GetMovementTreshold)))
            (bind _asbp_character_m_2 (Utilities|Casting|CastToBP_Character_M (Game|Player|GetPlayerPawn 0)))
            (Default|RotateCameratoLeft _asbp_character_m_2)
            (Variables|Default|SetIsTouchActive false)))))))

(fn ConstructionScript)